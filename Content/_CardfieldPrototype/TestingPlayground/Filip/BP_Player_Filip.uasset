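; Prototype player camera pawn for the card field, with pan, zoom and 45-degree step rotation.
; Input sets desired location, rotation and clamped arm length, which Tick interpolates toward.
; Key 1 toggles instantly between the starting transform and an offset, 180-degree-turned opposite view.
; The controller's OnPlayerChange event flips the sign of PlayerMultiplier, which is not otherwise used here.
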(event Custom|ChangePlayerMultiplier
  (Variables|Default|SetPlayerMultiplier (* (Variables|Default|GetPlayerMultiplier) -1.0)))

(event EventTick
  (params (DeltaSeconds :type Float%20%28single-precision%29))
  (bind _springarm (Variables|Default|GetSpringArm))
  (Variables|/Script/Engine.SpringArmComponent|SetTargetArmLength _springarm (Math|Interpolation|FInterpTo (Variables|/Script/Engine.SpringArmComponent|GetTargetArmLength _springarm) (Variables|Default|GetZoom_Desired) DeltaSeconds (Variables|Default|GetZoomInterpSpeed)))
  (Transformation|SetActorLocation (Math|Interpolation|VInterpTo (Transformation|GetActorLocation) (Variables|Default|GetLocationDesired) DeltaSeconds (Variables|Default|GetMoveInterpSpeed)) false false)
  (Transformation|SetActorRotation (Math|Interpolation|RInterpTo (Transformation|GetActorRotation) (Variables|Default|GetRotationDesired) DeltaSeconds (Variables|Default|GetRotationInterpSpeed))))

(event EventBeginPlay
  (bind _output_get (Variables|Default|SetInitialTransform (Transformation|GetActorTransform)))
  (Variables|Default|SetMirroredTransform (Math|Transform|MakeTransform (+ (.Location (Math|Transform|BreakTransform _output_get)) "-1300.000000,0.000000,0.000000") (Math|Rotator|CombineRotators (.Rotation (Math|Transform|BreakTransform _output_get)) "0.000000,-180.000000,0.000000") (.Scale (Math|Transform|BreakTransform _output_get))))
  (bind _aspc_controller_filip (Utilities|Casting|CastToPC_Controller_Filip (Pawn|GetController)))
  (EventDispatchers|BindEventtoOnPlayerChange _aspc_controller_filip (delegate Custom|ChangePlayerMultiplier))
  (Transformation|SetActorRotation (Transformation|GetActorRotation))
  (Variables|Default|SetLocationDesired (Transformation|GetActorLocation))
  (Variables|Default|SetZoom_Desired (Variables|/Script/Engine.SpringArmComponent|GetTargetArmLength (Variables|Default|GetSpringArm))))

(event Input|ActionEvents|InputActionInputAction_RotationRight
  (params (Key :type Key%20Structure :default "None"))
  (:Pressed
    (Variables|Default|SetRotationDesired (Math|Rotator|CombineRotators (Variables|Default|GetRotationDesired) "0.000000,-45.000000,0.000000"))))

(event Input|ActionEvents|InputActionInputAction_RotationLeft
  (params (Key :type Key%20Structure :default "None"))
  (:Pressed
    (Variables|Default|SetRotationDesired (Math|Rotator|CombineRotators (Variables|Default|GetRotationDesired) "0.000000,45.000000,0.000000"))))

(event Input|AxisEvents|InputAxisInputAxis_Forward
  (params (AxisValue :type Float%20%28single-precision%29))
  (Variables|Default|SetLocationDesired (+ (Variables|Default|GetLocationDesired) (* (Transformation|GetActorForwardVector) (* AxisValue (Variables|Default|GetMoveSpeed))))))

(event Input|AxisEvents|InputAxisInputAxis_Right
  (params (AxisValue :type Float%20%28single-precision%29))
  (Variables|Default|SetLocationDesired (+ (Variables|Default|GetLocationDesired) (* (Transformation|GetActorRightVector) (* AxisValue (Variables|Default|GetMoveSpeed))))))

(event Input|AxisEvents|InputAxisInputAxisZoom
  (params (AxisValue :type Float%20%28single-precision%29))
  (Variables|Default|SetZoom_Desired (Math|Float|Clamp(Float) (+ (* AxisValue (Variables|Default|GetZoomSpeed)) (Variables|Default|GetZoom_Desired)) (Variables|Default|GetMinZoom) (Variables|Default|GetMaxZoom))))

(event Input|KeyboardEvents|1
  (params (Key :type Key%20Structure :default "None"))
  (bind _mirroredtransform (Variables|Default|GetMirroredTransform))
  (bind _initialtransform (Variables|Default|GetInitialTransform))
  (bind (_location _rotation) (Math|Transform|BreakTransform _initialtransform))
  (bind (_location_2 _rotation_2) (Math|Transform|BreakTransform _mirroredtransform))
  (:Pressed
    (Variables|Default|SetZoom_Desired (Variables|/Script/Engine.SpringArmComponent|GetTargetArmLength (Variables|Default|GetSpringArm)))
    (Utilities|FlowControl|FlipFlop
      (:A
        (Variables|Default|SetRotationDesired _rotation_2)
        (Variables|Default|SetLocationDesired _location_2)
        (Transformation|SetActorTransform (Variables|Default|GetMirroredTransform)))
      (:B
        (Variables|Default|SetRotationDesired _rotation)
        (Variables|Default|SetLocationDesired _location)
        (Transformation|SetActorTransform (Variables|Default|GetInitialTransform))))))

(fn ConstructionScript)