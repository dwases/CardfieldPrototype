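; Prototype player controller for a two-player, turn-based card battle on a slot grid, tracking whose turn it is, resources and shared Nexus health.
; A state machine drives mouse input: left-drag draws a movement path through MapManager, right-click starts attack targeting.
; Paths show straight or turned line materials via a direction-pair lookup, with a timer-delayed attack-range preview.
; Turn changes restore every card's speed and attack.
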(event Custom|OnPlayerChange_Event
  (Development|PrintString "EventTest"))

(event Custom|CustomEvent
  (bind _returnvalue (Game|Player|GetPlayerPawn 0))
  (bind _returnvalue_2 (Actor|GetComponentbyClass _returnvalue "/Script/Engine.CameraComponent"))
  ;[0.15 0.15 0.15 0.5] backup - change player i enhanced input action ia_change player
  (Default|CallOnPlayerChange)
  (Utilities|FlowControl|FlipFlop
    (:A
      (Transformation|SetWorldRotation _returnvalue_2 "-66.000000,0.000000,0.000000" false false)
      (Transformation|AddRelativeLocation _returnvalue_2 "-1300.000000,0.000000,0.000000" false false)
      (Variables|Default|SetPlayerOneTurn false))
    (:B
      (Transformation|SetWorldRotation _returnvalue_2 "-66.000000,180.000000,0.000000" false false)
      (Transformation|AddRelativeLocation _returnvalue_2 "1300.000000,0.000000,0.000000" false false)
      (Variables|Default|SetPlayerOneTurn true))))

(event Custom|Shortcut%20to%20Drawing%20Line
  (bind _array (Utilities|Array|MakeArray "ObjectTypeQuery7"))
  (bind _hitresult (Class|PlayerController|GetHitResultUnderCursorforObjects _array false))
  (bind _hitactor (Collision|BreakHitResult _hitresult))
  (Utilities|IsValid _hitactor
    (:Is%20Valid
      (bind _asbp_card (Utilities|Casting|CastToBP_Card _hitactor)) ; For prototype
      (if (== (Variables|/Game/_CardfieldPrototype/TestingPlayground/Filip/Card/BP_Card.BP_Card_C|GetbPlayerOne _asbp_card) (Variables|Default|GetPlayerOneTurn))
        (bind _output_get (Variables|Default|SetSelectedCard _asbp_card))
        (Development|PrintString "Card selected")
        (if (> (Variables|/Game/_CardfieldPrototype/TestingPlayground/Filip/Card/BPC_StatsComponent.BPC_StatsComponent_C|GetSpeedLeft (Variables|/Game/_CardfieldPrototype/TestingPlayground/Filip/Card/BP_Card.BP_Card_C|GetBPC_StatsComponent _output_get)) 0)
          (Variables|Default|SetState "NewEnumerator1")
          (Utilities|Array|Clear (Variables|Default|GetSlotArray_CurrentLine))
          (CallFunction|ClearCurrentLine true)
          (Utilities|Array|Add (Variables|Default|GetSlotArray_CurrentLine) (Variables|/Game/_CardfieldPrototype/TestingPlayground/Filip/Card/BP_Card.BP_Card_C|GetmySlot (Variables|Default|GetSelectedCard))))))))

(event Custom|ChangePlayer
  (Default|CallOnPlayerChange)
  (Utilities|FlowControl|FlipFlop
    (:A
      (Variables|Default|SetPlayerOneTurn false))
    (:B
      (Variables|Default|SetPlayerOneTurn true)))
  (bind _outactors (Actor|GetAllActorsOfClass "/Game/_CardfieldPrototype/TestingPlayground/Filip/Card/BP_Card.BP_Card_C"))
  (for _array_element _outactors
    (Variables|/Game/_CardfieldPrototype/TestingPlayground/Filip/Card/BP_Card.BP_Card_C|SetbUsedAttack _array_element false)
    (Default|RestoreSpeed (Variables|/Game/_CardfieldPrototype/TestingPlayground/Filip/Card/BP_Card.BP_Card_C|GetBPC_StatsComponent _array_element))))

(event Custom|Start%20Moving
  (Variables|Default|SetState "NewEnumerator2")
  (bind _arrayout (CallFunction|ClipFirstIndex (Variables|Default|GetSlotArray_CurrentLine)))
  (Default|Move (Variables|Default|GetSelectedCard) _arrayout)
  (Utilities|Array|Clear (Variables|Default|GetSlotArray_CurrentLine)))

(event Custom|Printer
  (bind _resources (Variables|Default|GetResources))
  (bind (_materials _energy _minerals) (Utilities|Struct|BreakS_Resources _resources))
  (Development|PrintText (Utilities|Text|FormatText "Nexus HP: {X}" (Variables|Default|GetNexusHealth)) true false "(R=0.000000,G=1.000000,B=0.131262,A=1.000000)" 2.0 "nHP")
  (Development|PrintText (Utilities|Text|FormatText "Materials: {X}  
Energy: {Y} 
Minerals: {Z}" _materials _energy _minerals) true false "(R=0.700777,G=0.127206,B=1.000000,A=1.000000)" 2.0 "Res"))

(event Input|EnhancedActionEvents|EnhancedInputActionIA_LeftClick
  (params (ActionValue :type Boolean) (ElapsedSeconds :type Float%20%28double-precision%29) (TriggeredSeconds :type Float%20%28double-precision%29) (InputAction :type Input%20Action%20Object%20Reference :default "/Game/_CardfieldPrototype/TestingPlayground/Filip/Input/IA_LeftClick.IA_LeftClick"))
  (bind _array (Utilities|Array|MakeArray "ObjectTypeQuery7"))
  (bind _array_2 (Utilities|Array|MakeArray "ObjectTypeQuery8"))
  (bind _array_3 (Utilities|Array|MakeArray "ObjectTypeQuery7"))
  (bind _hitresult (Class|PlayerController|GetHitResultUnderCursorforObjects _array false))
  (bind (_hitresult_2 _returnvalue) (Class|PlayerController|GetHitResultUnderCursorforObjects _array_2 false))
  (bind (_hitresult_3 _returnvalue_2) (Class|PlayerController|GetHitResultUnderCursorforObjects _array_3 true))
  (bind _hitactor (Collision|BreakHitResult _hitresult))
  (:Started
    (switch Utilities|FlowControl|Switch|SwitchonE_ControllerState (Variables|Default|GetState)
      (:NewEnumerator0
        (Utilities|IsValid _hitactor :!label _label
          (:Is%20Valid
            (bind _asbp_card (Utilities|Casting|CastToBP_Card _hitactor)) ; For prototype
            (if (== (Variables|/Game/_CardfieldPrototype/TestingPlayground/Filip/Card/BP_Card.BP_Card_C|GetbPlayerOne _asbp_card) (Variables|Default|GetPlayerOneTurn))
              (bind _output_get (Variables|Default|SetSelectedCard _asbp_card))
              (Development|PrintString "Card selected")
              (if (> (Variables|/Game/_CardfieldPrototype/TestingPlayground/Filip/Card/BPC_StatsComponent.BPC_StatsComponent_C|GetSpeedLeft (Variables|/Game/_CardfieldPrototype/TestingPlayground/Filip/Card/BP_Card.BP_Card_C|GetBPC_StatsComponent _output_get)) 0)
                (Variables|Default|SetState "NewEnumerator1")
                (Utilities|Array|Clear (Variables|Default|GetSlotArray_CurrentLine))
                (CallFunction|ClearCurrentLine true)
                (Utilities|Array|Add (Variables|Default|GetSlotArray_CurrentLine) (Variables|/Game/_CardfieldPrototype/TestingPlayground/Filip/Card/BP_Card.BP_Card_C|GetmySlot (Variables|Default|GetSelectedCard))))))))
      (:NewEnumerator4
        (if _returnvalue_2
          (bind _asbp_card_2 (Utilities|Casting|CastToBP_Card (.HitActor (Collision|BreakHitResult _hitresult_3))))
          (if (== (Variables|/Game/_CardfieldPrototype/TestingPlayground/Filip/Card/BP_Card.BP_Card_C|GetbPlayerOne _asbp_card_2) (Variables|Default|GetPlayerOneTurn))
            (bind _slots (Default|ConvertMasktoMap (Variables|Default|GetMapManager) (Variables|/Game/_CardfieldPrototype/TestingPlayground/Filip/Card/BP_Card.BP_Card_C|GetmySlot (Variables|Default|GetSelectedCard)) (Variables|/Game/_CardfieldPrototype/TestingPlayground/Filip/Card/BP_Card.BP_Card_C|GetMaskAttack (Variables|Default|GetSelectedCard))))
            (for _array_element _slots
              (bind _asbp_slot (Utilities|Casting|CastToBP_Slot _array_element))
              (Default|AttackMaterialOFF _asbp_slot))
            (CallFunction|ShortcuttoDrawingLine)
            (else
              (if _returnvalue :!label _label_2
                (bind _asbp_slot_2 (Utilities|Casting|CastToBP_Slot (.HitActor (Collision|BreakHitResult _hitresult_2))))
                (Variables|/Game/_CardfieldPrototype/TestingPlayground/Filip/Slot/BP_Slot.BP_Slot_C|GetAttackable _asbp_slot_2
                  (:then
                    (Utilities|IsValid (Variables|/Game/_CardfieldPrototype/TestingPlayground/Filip/Slot/BP_Slot.BP_Slot_C|GetCard _asbp_slot_2)
                      (:Is%20Valid
                        (CallFunction|Attack (Variables|Default|GetSelectedCard) (Variables|/Game/_CardfieldPrototype/TestingPlayground/Filip/Slot/BP_Slot.BP_Slot_C|GetCard _asbp_slot_2)))
                      (:Is%20Not%20Valid
                        (CallFunction|Attack (Variables|Default|GetSelectedCard) 0 _asbp_slot_2)))
                    (bind _slots_2 (Default|ConvertMasktoMap (Variables|Default|GetMapManager) (Variables|/Game/_CardfieldPrototype/TestingPlayground/Filip/Card/BP_Card.BP_Card_C|GetmySlot (Variables|Default|GetSelectedCard)) (Variables|/Game/_CardfieldPrototype/TestingPlayground/Filip/Card/BP_Card.BP_Card_C|GetMaskAttack (Variables|Default|GetSelectedCard))))
                    (for _array_element_2 _slots_2
                      (bind _asbp_slot_3 (Utilities|Casting|CastToBP_Slot _array_element_2))
                      (Default|AttackMaterialOFF _asbp_slot_3))
                    (Default|SetMaskAttack (Variables|Default|GetSelectedCard))
                    (Variables|/Game/_CardfieldPrototype/TestingPlayground/Filip/Card/BP_Card.BP_Card_C|SetbUsedAttack (Variables|Default|GetSelectedCard) true)
                    (bind _aswbp_card (Utilities|Casting|CastToWBP_Card (UserInterface|GetWidget (Variables|/Game/_CardfieldPrototype/TestingPlayground/Filip/Card/BP_Card.BP_Card_C|GetWidget (Variables|Default|GetSelectedCard)))))
                    (Default|UpdateCardStats _aswbp_card 0 (Variables|Default|GetSelectedCard)))
                  (:else)))))
          (else
            (goto _label_2))))
      (:NewEnumerator6
        (goto _label))))
  (:Completed
    (switch Utilities|FlowControl|Switch|SwitchonE_ControllerState (Variables|Default|GetState)
      (:NewEnumerator1
        (Variables|Default|SetState "NewEnumerator0")
        (CallFunction|ToggleMask)
        (CallFunction|StartMoving)
        (Variables|Default|SetLastSlotUsedForMask 0)))))

(event Input|EnhancedActionEvents|EnhancedInputActionIA_RightClick
  (params (ActionValue :type Boolean) (ElapsedSeconds :type Float%20%28double-precision%29) (TriggeredSeconds :type Float%20%28double-precision%29) (InputAction :type Input%20Action%20Object%20Reference :default "/Game/_CardfieldPrototype/TestingPlayground/Filip/Input/IA_RightClick.IA_RightClick"))
  (bind _array (Utilities|Array|MakeArray "ObjectTypeQuery7"))
  (bind _array_2 (Utilities|Array|MakeArray "ObjectTypeQuery7"))
  (bind _hitresult (Class|PlayerController|GetHitResultUnderCursorforObjects _array_2 false))
  (bind (_hitresult_2 _returnvalue) (Class|PlayerController|GetHitResultUnderCursorforObjects _array false))
  (bind _hitactor (Collision|BreakHitResult _hitresult))
  (bind _hitactor_2 (Collision|BreakHitResult _hitresult_2))
  (switch Utilities|FlowControl|Switch|SwitchonE_ControllerState (Variables|Default|GetState)
    (:NewEnumerator0
      (Utilities|IsValid _hitactor :!label _label
        (:Is%20Valid
          (bind _asbp_card (Utilities|Casting|CastToBP_Card _hitactor)) ; For prototype
          (if (== (Variables|Default|GetPlayerOneTurn) (Variables|/Game/_CardfieldPrototype/TestingPlayground/Filip/Card/BP_Card.BP_Card_C|GetbPlayerOne _asbp_card))
            (bind _output_get (Variables|Default|SetSelectedCard _asbp_card))
            (Variables|/Game/_CardfieldPrototype/TestingPlayground/Filip/Card/BP_Card.BP_Card_C|GetbUsedAttack _output_get
              (:then)
              (:else
                (bind _slots (Default|ConvertMasktoMap (Variables|Default|GetMapManager) (Variables|/Game/_CardfieldPrototype/TestingPlayground/Filip/Card/BP_Card.BP_Card_C|GetmySlot (Variables|Default|GetSelectedCard)) (Variables|/Game/_CardfieldPrototype/TestingPlayground/Filip/Card/BP_Card.BP_Card_C|GetMaskAttack (Variables|Default|GetSelectedCard))))
                (for _array_element _slots
                  (bind _asbp_slot (Utilities|Casting|CastToBP_Slot _array_element))
                  (Default|AttackMaterialON _asbp_slot false)
                  (Variables|Default|SetState "NewEnumerator4"))))))))
    (:NewEnumerator1
      (Variables|Default|SetState "NewEnumerator0")
      (CallFunction|ClearCurrentLine false)
      (CallFunction|ToggleMask)
      (Variables|Default|SetLastSlotUsedForMask 0))
    (:NewEnumerator4
      (if _returnvalue
        (bind _asbp_card_2 (Utilities|Casting|CastToBP_Card _hitactor_2))
        (if (== (Variables|/Game/_CardfieldPrototype/TestingPlayground/Filip/Card/BP_Card.BP_Card_C|GetbPlayerOne _asbp_card_2) (Variables|Default|GetPlayerOneTurn))
          (bind _slots_2 (Default|ConvertMasktoMap (Variables|Default|GetMapManager) (Variables|/Game/_CardfieldPrototype/TestingPlayground/Filip/Card/BP_Card.BP_Card_C|GetmySlot (Variables|Default|GetSelectedCard)) (Variables|/Game/_CardfieldPrototype/TestingPlayground/Filip/Card/BP_Card.BP_Card_C|GetMaskAttack (Variables|Default|GetSelectedCard))))
          (for _array_element_2 _slots_2
            (bind _asbp_slot_2 (Utilities|Casting|CastToBP_Slot _array_element_2))
            (Default|AttackMaterialOFF _asbp_slot_2))
          (if (== _hitactor_2 (Variables|Default|GetSelectedCard))
            (Variables|Default|SetSelectedCard 0)
            (else
              (goto _label))))))))

(event Input|EnhancedActionEvents|EnhancedInputActionIA_ChangePlayer
  (params (ActionValue :type Boolean) (ElapsedSeconds :type Float%20%28double-precision%29) (TriggeredSeconds :type Float%20%28double-precision%29) (InputAction :type Input%20Action%20Object%20Reference :default "/Game/_CardfieldPrototype/TestingPlayground/Filip/Input/IA_ChangePlayer.IA_ChangePlayer"))
  (bind _returnvalue (Game|Player|GetPlayerPawn 0))
  (bind _returnvalue_2 (Actor|GetComponentbyClass _returnvalue "/Script/Engine.CameraComponent"))
  ;[0.15 0.15 0.15 0.5] backup - change player i enhanced input action ia_change player
  (Default|CallOnPlayerChange)
  (Utilities|FlowControl|FlipFlop
    (:A
      (Transformation|SetWorldRotation _returnvalue_2 "-66.000000,0.000000,0.000000" false false)
      (Transformation|AddRelativeLocation _returnvalue_2 "-1300.000000,0.000000,0.000000" false false)
      (Variables|Default|SetPlayerOneTurn false))
    (:B
      (Transformation|SetWorldRotation _returnvalue_2 "-66.000000,180.000000,0.000000" false false)
      (Transformation|AddRelativeLocation _returnvalue_2 "1300.000000,0.000000,0.000000" false false)
      (Variables|Default|SetPlayerOneTurn true))))

(event Input|EnhancedActionEvents|EnhancedInputActionIA_ChangePlayer
  (params (ActionValue :type Boolean) (ElapsedSeconds :type Float%20%28double-precision%29) (TriggeredSeconds :type Float%20%28double-precision%29) (InputAction :type Input%20Action%20Object%20Reference :default "/Game/_CardfieldPrototype/TestingPlayground/Filip/Input/IA_ChangePlayer.IA_ChangePlayer"))
  (Default|CallOnPlayerChange)
  (Utilities|FlowControl|FlipFlop
    (:A
      (Variables|Default|SetPlayerOneTurn false))
    (:B
      (Variables|Default|SetPlayerOneTurn true)))
  (bind _outactors (Actor|GetAllActorsOfClass "/Game/_CardfieldPrototype/TestingPlayground/Filip/Card/BP_Card.BP_Card_C"))
  (for _array_element _outactors
    (Variables|/Game/_CardfieldPrototype/TestingPlayground/Filip/Card/BP_Card.BP_Card_C|SetbUsedAttack _array_element false)
    (Default|RestoreSpeed (Variables|/Game/_CardfieldPrototype/TestingPlayground/Filip/Card/BP_Card.BP_Card_C|GetBPC_StatsComponent _array_element))))

(event EventBeginPlay
  (bind _returnvalue (PlayerController|LocalPlayerSubsystems|GetEnhancedInputLocalPlayerSubsystem))
  (Variables|Default|SetbShowMouseCursor true)
  (Utilities|IsValid _returnvalue
    (:Is%20Valid
      (Input|AddMappingContext _returnvalue "/Game/_CardfieldPrototype/TestingPlayground/Filip/Input/IMP_KeyMapping.IMP_KeyMapping" 0 "(bIgnoreAllPressedKeysUntilRelease=True,bForceImmediately=False,bNotifyUserSettings=False)")
      (bind _returnvalue_2 (Actor|GetActorOfClass "/Game/_CardfieldPrototype/TestingPlayground/Filip/Slot/BP_MapManager.BP_MapManager_C")) ; Prototype == HardRef
      (Variables|Default|SetMapManager _returnvalue_2)
      (Utilities|Time|SetTimerbyEvent (delegate Custom|Printer) 0.25 true))))

(event EventTick
  (params (DeltaSeconds :type Float%20%28single-precision%29))
  (bind _array (Utilities|Array|MakeArray "ObjectTypeQuery8"))
  (bind _slotarray_currentline (Variables|Default|GetSlotArray_CurrentLine))
  (bind _hitresult (Class|PlayerController|GetHitResultUnderCursorforObjects _array false))
  (bind _hitactor (Collision|BreakHitResult _hitresult))
  (switch Utilities|FlowControl|Switch|SwitchonE_ControllerState (Variables|Default|GetState)
    (:NewEnumerator1
      (Utilities|IsValid _hitactor
        (:Is%20Valid
          (if (not (== (Variables|Default|GetLastSlotUsedForMask) _hitactor))
            (CallFunction|ToggleMask)
            (Variables|Default|SetLastSlotUsedForMask _hitactor)
            (bind _result (Default|DoPathifPossible (Variables|Default|GetMapManager) _hitactor (Variables|Default|GetSlotArray_CurrentLine)))
            (if (not (Utilities|Array|Identical _result (Variables|Default|GetSlotArray_CurrentLine)))
              (CallFunction|ClearCurrentLine false)
              (if (not (Utilities|Array|IsEmpty _result))
                ;[0.15 0.15 0.15 0.5] Temp -> Protytpe == HardRef
                (bind _array_element (Utilities|Array|ForEachLoopwithBreak _result)
                  (:LoopBody
                    (Utilities|Array|AddUnique (Variables|Default|GetSlotArray_CurrentLine) _array_element))
                  (:Completed
                    (CallFunction|UpdateLineVisuals _slotarray_currentline)
                    (bind _arrayout (CallFunction|ClipFirstIndex _slotarray_currentline))
                    (CallFunction|ToggleMask _arrayout)))))))))))

(event EventAddCardtoPlayerCards
  (params (Card :type Actor%20Object%20Reference))
  (Utilities|Array|Add (Variables|Default|GetPlayerCards) Card))

(fn ConstructionScript)

(fn DrawLine
  (params (Array :type Array%20of%20Actor%20Object%20References))
  (bind _selectedcard (Variables|Default|GetSelectedCard))
  (for _array_element Array
    (bind _asbp_slot (Utilities|Casting|CastToBP_Slot _array_element))
    (Utilities|Array|Add (LocalVariables|GetTempRef) _asbp_slot))
  (for _array_element_2 (LocalVariables|GetTempRef)
    (Default|LineMaterial _array_element_2 0.0 false false))
  (Utilities|Map|Add (Variables|Default|GetLines) _selectedcard (Utilities|Struct|MakeS_Lines _selectedcard (LocalVariables|GetTempRef))))

(fn ClearCurrentLine
  (params (Old :type Boolean))
  (bind _selectedcard (Variables|Default|GetSelectedCard))
  (bind _selectedcard_2 (Variables|Default|GetSelectedCard))
  (if Old
    (Variables|Default|SetSlotArray_CurrentLine (.array (.Value (Utilities|Map|Find (Variables|Default|GetLines) (Variables|Default|GetSelectedCard)))))
    (for _array_element (Variables|Default|GetSlotArray_CurrentLine)
      (Class|BPItoSlot|SetDefaultMaterial(Message) _array_element))
    (Utilities|Array|Clear (Variables|Default|GetSlotArray_CurrentLine))
    (Utilities|Map|Add (Variables|Default|GetLines) _selectedcard_2 (Utilities|Struct|MakeS_Lines _selectedcard_2 (Utilities|Array|MakeArray)))
    (else
      (for _array_element_2 (Variables|Default|GetSlotArray_CurrentLine)
        (Class|BPItoSlot|SetDefaultMaterial(Message) _array_element_2))
      (Utilities|Array|Clear (Variables|Default|GetSlotArray_CurrentLine))
      (Utilities|Map|Add (Variables|Default|GetLines) _selectedcard (Utilities|Struct|MakeS_Lines _selectedcard (Utilities|Array|MakeArray))))))

(fn Attack
  (params (Card :type Actor%20Object%20Reference) (Target :type Actor%20Object%20Reference) (TargetSlot%20%28Optional%29 :type Actor%20Object%20Reference))
  (bind _asbp_card (Utilities|Casting|CastToBP_Card Card))
  (bind _asbp_card_2 (Utilities|Casting|CastToBP_Card Target)
    (:then
      (Default|TakeDamage _asbp_card_2 (Variables|/Game/_CardfieldPrototype/TestingPlayground/Filip/Card/PDA_CardStats.PDA_CardStats_C|GetAttack (Variables|/Game/_CardfieldPrototype/TestingPlayground/Filip/Card/BP_Card.BP_Card_C|GetStats _asbp_card))))
    (:CastFailed
      (bind _asbp_slot (Utilities|Casting|CastToBP_Slot TargetSlot%20%28Optional%29))
      ;[0.15 0.15 0.15 0.5] Prototype - for now there is only one Nexus HP for both Players
      (Variables|/Game/_CardfieldPrototype/TestingPlayground/Filip/Slot/BP_Slot.BP_Slot_C|GetBaseSlot _asbp_slot
        (:then
          (Variables|Default|SetNexusHealth (- (Variables|Default|GetNexusHealth) (Variables|/Game/_CardfieldPrototype/TestingPlayground/Filip/Card/PDA_CardStats.PDA_CardStats_C|GetAttack (Variables|/Game/_CardfieldPrototype/TestingPlayground/Filip/Card/BP_Card.BP_Card_C|GetStats _asbp_card)))))
        (:else)))))

(fn PayforAction
  (params (Materials :type Integer) (Energy :type Integer) (Minerals :type Integer))
  (if (Math|Boolean|ANDBoolean (<= Materials (.Materials (Utilities|Struct|BreakS_Resources (Variables|Default|GetResources)))) (<= Energy (.Energy (Utilities|Struct|BreakS_Resources (Variables|Default|GetResources)))) (<= Minerals (.Minerals (Utilities|Struct|BreakS_Resources (Variables|Default|GetResources)))))
    (Variables|Default|SetResources (Utilities|Struct|MakeS_Resources (- (.Materials (Utilities|Struct|BreakS_Resources (Variables|Default|GetResources))) Materials) (- (.Energy (Utilities|Struct|BreakS_Resources (Variables|Default|GetResources))) Energy) (- (.Minerals (Utilities|Struct|BreakS_Resources (Variables|Default|GetResources))) Minerals)))
    (return true)
    (else
      (return false))))

(fn SetControllerState
  (params (State :type E_ControllerState%20Enum :default "NewEnumerator0"))
  (bind _output_get (Variables|Default|SetState State))
  (switch Utilities|FlowControl|Switch|SwitchonE_ControllerState _output_get) ; Funkcjonalny Setter na przyszlość
)

(fn ClipFirstIndex
  (params (ArrayIn :type Array%20of%20Actor%20Object%20References))
  (bind _output_get (LocalVariables|SetTemp ArrayIn))
  (Utilities|Array|RemoveIndex _output_get)
  (return (LocalVariables|GetTemp)))

(fn UpdateLineVisuals
  (params (Path :type Array%20of%20Actor%20Object%20References))
  (if (> (Utilities|Array|Length Path) 1)
    (for _array_element Path
      (bind _asbp_slot (Utilities|Casting|CastToBP_Slot _array_element))
      (Utilities|Array|Add (LocalVariables|GetTempCast) _asbp_slot))
    (for _index (range 0 (- (Utilities|Array|Length (LocalVariables|GetTempCast)) 1))
      (LocalVariables|SetIndex _index)
      (if (> (LocalVariables|GetIndex) 0)
        (LocalVariables|SetPrev (Utilities|Array|Get(acopy) (LocalVariables|GetTempCast) (- (LocalVariables|GetIndex) 1))))
      (LocalVariables|SetCurrent (Utilities|Array|Get(acopy) (LocalVariables|GetTempCast) (LocalVariables|GetIndex)))
      (if (< (LocalVariables|GetIndex) (- (Utilities|Array|Length (LocalVariables|GetTempCast)) 1))
        (LocalVariables|SetNext (Utilities|Array|Get(acopy) (LocalVariables|GetTempCast) (+ (LocalVariables|GetIndex) 1))))
      (if (== (LocalVariables|GetIndex) (- (Utilities|Array|Length (LocalVariables|GetTempCast)) 1)) ; Ostatni Index,\nSlot Next jest Invalid
        (LocalVariables|SetRot (CallFunction|DirtoRotVisuals (Default|GetDir (Variables|Default|GetMapManager) (LocalVariables|GetPrev) (LocalVariables|GetCurrent))))
        (Default|LineMaterial (Utilities|Array|Get(acopy) (LocalVariables|GetTempCast) (LocalVariables|GetIndex)) (LocalVariables|GetRot) false false :!label _label)
        (elif (not (== (LocalVariables|GetIndex) 0)) ; Skip na 0
          (LocalVariables|SetDirIN (Default|GetDir (Variables|Default|GetMapManager) (LocalVariables|GetPrev) (LocalVariables|GetCurrent)))
          (LocalVariables|SetDirOUT (Default|GetDir (Variables|Default|GetMapManager) (LocalVariables|GetCurrent) (LocalVariables|GetNext)))
          (if (Utilities|Enum|Equal(Enum) (LocalVariables|GetDirIN) (LocalVariables|GetDirOUT))
            (LocalVariables|SetRot (CallFunction|DirtoRotVisuals (LocalVariables|GetDirOUT)))
            (goto _label)
            (else
              (Default|LineMaterial (Utilities|Array|Get(acopy) (LocalVariables|GetTempCast) (LocalVariables|GetIndex)) (.Rotation (CallFunction|TurntoRotVisuals (LocalVariables|GetDirIN) (LocalVariables|GetDirOUT))) true (.Mirror (CallFunction|TurntoRotVisuals (LocalVariables|GetDirIN) (LocalVariables|GetDirOUT)))))))))))

(fn DirtoRotVisuals
  (params (Direction :type EDirection%20Enum :default "Left"))
  (return (Utilities|Select :Index Direction :Left 0.5 :Right 0.0 :Up 0.25 :Down 0.75 :Front 0.0 :Back 0.0)))

(fn TurntoRotVisuals
  (params (DirIN :type EDirection%20Enum :default "Left") (DirOUT :type EDirection%20Enum :default "Left"))
  (bind _id (CallFunction|ConvertDirtoID DirOUT))
  (bind _id_2 (CallFunction|ConvertDirtoID DirIN))
  (bind _map (LocalVariables|GetMap))
  (bind _returnvalue (* _id_2 4))
  (bind _returnvalue_2 (+ _returnvalue _id))
  (bind _value (Utilities|Map|Find _map _returnvalue_2))
  (Development|PrintString (Utilities|String|ToString(Integer) _returnvalue_2) true true "(R=0.000000,G=0.660000,B=1.000000,A=1.000000)" 2.0 "abccccc")
  (return (.rot _value) (.mirror _value)))

(fn ConvertDirtoID
  (params (Dir :type EDirection%20Enum :default "Left"))
  (return (Utilities|Select :Index Dir :Left 3 :Right 1 :Up 0 :Down 2 :Front 0 :Back 0)))

(fn ToggleMask
  (params (Path :type Array%20of%20Actor%20Object%20References))
  (Utilities|IsValid (Variables|Default|GetLastSlotUsedForMask)
    (:Is%20Valid
      (bind _slots (Default|ConvertMasktoMap (Variables|Default|GetMapManager) (Variables|Default|GetLastSlotUsedForMask) (Variables|/Game/_CardfieldPrototype/TestingPlayground/Filip/Card/BP_Card.BP_Card_C|GetMaskAttack (Variables|Default|GetSelectedCard))))
      (for _array_element _slots
        (bind _asbp_slot (Utilities|Casting|CastToBP_Slot _array_element))
        (Default|AttackMaterialOFF _asbp_slot)))
    (:Is%20Not%20Valid
      _))
  (if (not (Utilities|Array|IsEmpty Path))
    (Default|ConvertMasktoMap (Variables|Default|GetMapManager) (Utilities|Array|Get(acopy) Path (Utilities|Array|LastIndex Path)) (Variables|/Game/_CardfieldPrototype/TestingPlayground/Filip/Card/BP_Card.BP_Card_C|GetMaskAttack (Variables|Default|GetSelectedCard)))
    (Variables|Default|SetLastSlotUsedForMask (Utilities|Array|Get(acopy) Path (Utilities|Array|LastIndex Path)))
    (Utilities|Time|SetTimerbyFunctionName 0 "Validate Threshold" 0.4)))

(fn PassivelyGainBattleResources
  (bind _resourcesperturn (Variables|Default|GetResourcesPerTurn))
  (Variables|Default|SetResources (Utilities|Struct|MakeS_Resources (+ (.materials (Variables|Default|GetResources)) (.materials _resourcesperturn)) (+ (.energy (Variables|Default|GetResources)) (.energy _resourcesperturn)) (+ (.minerals (Variables|Default|GetResources)) (.minerals _resourcesperturn)))))

(fn IncreaseResourcePassiveGain
  (params (ResourceName :type String))
  (if (Utilities|Enum|Equal(Enum) ResourceName "Materials")
    (Utilities|Struct|SetmembersinS_Resources (Variables|Default|GetResourcesPerTurn) (+ (.materials (Variables|Default|GetResourcesPerTurn)) 1))
    (elif (Utilities|Enum|Equal(Enum) ResourceName "Energy")
      (Utilities|Struct|SetmembersinS_Resources (Variables|Default|GetResourcesPerTurn) (+ (.energy (Variables|Default|GetResourcesPerTurn)) 1))
      (elif (Utilities|Enum|Equal(Enum) ResourceName "Minerals")
        (Utilities|Struct|SetmembersinS_Resources (Variables|Default|GetResourcesPerTurn) (+ (.minerals (Variables|Default|GetResourcesPerTurn)) 1))))))

(fn ValidateThreshold
  (bind _array (Utilities|Array|MakeArray "ObjectTypeQuery8"))
  (bind (_hitresult _returnvalue) (Class|PlayerController|GetHitResultUnderCursorforObjects _array false))
  (if _returnvalue
    (if (== (.HitActor (Collision|BreakHitResult _hitresult)) (Variables|Default|GetLastSlotUsedForMask))
      (bind _slots (Default|ConvertMasktoMap (Variables|Default|GetMapManager) (Variables|Default|GetLastSlotUsedForMask) (Variables|/Game/_CardfieldPrototype/TestingPlayground/Filip/Card/BP_Card.BP_Card_C|GetMaskAttack (Variables|Default|GetSelectedCard))))
      (for _array_element _slots
        (bind _asbp_slot (Utilities|Casting|CastToBP_Slot _array_element))
        (Default|AttackMaterialON _asbp_slot true)))))

(fn GetPlayerCards
  (return (Variables|Default|GetPlayerCards)))