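; Fog-of-war manager for the card grid, with one instanced mesh per map slot from BP_MapManager.
; RecalculateVisibility clears fog targets in a Manhattan-distance diamond around each card's vision and on base slots, then hides enemy cards in fogged slots.
; Tick eases each fog instance toward its target by scaling it.
; GetAndCalculateVisibility separately returns combined, base and card visibility maps, using either player or AI base slots.
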(event EventBeginPlay
  (bind _returnvalue (Actor|GetActorOfClass "/Game/_CardfieldPrototype/TestingPlayground/Filip/Slot/BP_MapManager.BP_MapManager_C"))
  (Variables|Default|SetMapManager _returnvalue)
  (Transformation|SetActorLocation "0.000000,0.000000,50.000000" false false)
  (CallFunction|InitFog)
  (Utilities|Array|Resize (Variables|Default|GetCurrentFade) (* (Variables|/Game/_CardfieldPrototype/TestingPlayground/Filip/Slot/BP_MapManager.BP_MapManager_C|GetWidth (Variables|Default|GetMapManager)) (Variables|/Game/_CardfieldPrototype/TestingPlayground/Filip/Slot/BP_MapManager.BP_MapManager_C|GetHeight (Variables|Default|GetMapManager))))
  (Utilities|Array|Resize (Variables|Default|GetTargetFade) (* (Variables|/Game/_CardfieldPrototype/TestingPlayground/Filip/Slot/BP_MapManager.BP_MapManager_C|GetWidth (Variables|Default|GetMapManager)) (Variables|/Game/_CardfieldPrototype/TestingPlayground/Filip/Slot/BP_MapManager.BP_MapManager_C|GetHeight (Variables|Default|GetMapManager))))
  (for _index (range 0 (- (* (Variables|/Game/_CardfieldPrototype/TestingPlayground/Filip/Slot/BP_MapManager.BP_MapManager_C|GetWidth (Variables|Default|GetMapManager)) (Variables|/Game/_CardfieldPrototype/TestingPlayground/Filip/Slot/BP_MapManager.BP_MapManager_C|GetHeight (Variables|Default|GetMapManager))) 1))
    (Utilities|Array|SetArrayElem (Variables|Default|GetCurrentFade) _index 1.0)
    (Utilities|Array|SetArrayElem (Variables|Default|GetTargetFade) _index 1.0)
    (Components|InstancedStaticMesh|SetCustomDataValue (Variables|Default|GetHISM_Fog) _index 0 1.0 true))
  (Utilities|FlowControl|DelayUntilNextTick)
  (Utilities|FlowControl|DelayUntilNextFrame)
  (bind _cards (Class|BPItoPlayer|GetPlayerCards(Message) (Game|GetPlayerController 0)))
  (CallFunction|RecalculateVisibility _cards))

(event EventTick
  (params (DeltaSeconds :type Float%20%28single-precision%29))
  (bind _hism_fog (Variables|Default|GetHISM_Fog))
  (bind _mapmanager (Variables|Default|GetMapManager))
  (Variables|Default|SetbNeedsUpdate false)
  (for _index (range 0 (- (* (Variables|/Game/_CardfieldPrototype/TestingPlayground/Filip/Slot/BP_MapManager.BP_MapManager_C|GetHeight _mapmanager) (Variables|/Game/_CardfieldPrototype/TestingPlayground/Filip/Slot/BP_MapManager.BP_MapManager_C|GetWidth _mapmanager)) 1))
    (Utilities|Array|SetArrayElem (Variables|Default|GetCurrentFade) _index (Math|Interpolation|FInterpTo (Utilities|Array|Get(acopy) (Variables|Default|GetCurrentFade) _index) (Utilities|Array|Get(acopy) (Variables|Default|GetTargetFade) _index) DeltaSeconds 4.0))
    (Components|InstancedStaticMesh|UpdateInstanceTransform _hism_fog _index (Math|Transform|MakeTransform (.location (.OutInstanceTransform (Components|InstancedStaticMesh|GetInstanceTransform _hism_fog _index true))) (.rotation (.OutInstanceTransform (Components|InstancedStaticMesh|GetInstanceTransform _hism_fog _index true))) (* "1.000000,1.000000,1.000000" (Utilities|Array|Get(acopy) (Variables|Default|GetCurrentFade) _index))) true true false)
    (if (> (Math|Float|Absolute(Float) (- (Utilities|Array|Get(acopy) (Variables|Default|GetCurrentFade) _index) (Utilities|Array|Get(acopy) (Variables|Default|GetTargetFade) _index))) 0.001)
      (Variables|Default|SetbNeedsUpdate true)))
  (Variables|Default|GetbNeedsUpdate
    (:then)
    (:else
      (Actor|Tick|SetActorTickEnabled false))))

(fn ConstructionScript)

(fn InitFog
  (for _index (range 1 (Variables|/Game/_CardfieldPrototype/TestingPlayground/Filip/Slot/BP_MapManager.BP_MapManager_C|GetWidth (Variables|Default|GetMapManager)))
    (LocalVariables|SetSpawnLocation (+ (Transformation|GetActorLocation (Variables|Default|GetMapManager)) (* (Math|Vector|MakeVector 0.0 (+ -1e+02 (Variables|/Game/_CardfieldPrototype/TestingPlayground/Filip/Slot/BP_MapManager.BP_MapManager_C|GetMargin (Variables|Default|GetMapManager))) 0.0) _index)))
    (for _index_2 (range 1 (Variables|/Game/_CardfieldPrototype/TestingPlayground/Filip/Slot/BP_MapManager.BP_MapManager_C|GetHeight (Variables|Default|GetMapManager)))
      (Components|InstancedStaticMesh|AddInstance (Variables|Default|GetHISM_Fog) (Math|Transform|MakeTransform (Math|Vector|MakeVector (+ (+ (.x (LocalVariables|GetSpawnLocation)) (Variables|/Game/_CardfieldPrototype/TestingPlayground/Filip/Slot/BP_MapManager.BP_MapManager_C|GetMargin (Variables|Default|GetMapManager))) -1.3e+02) (.y (LocalVariables|GetSpawnLocation)) (.z (LocalVariables|GetSpawnLocation))) "0, 0, 0" "1.000000,1.000000,1.000000") false)
      (LocalVariables|SetSpawnLocation (Math|Vector|MakeVector (+ (+ (.x (LocalVariables|GetSpawnLocation)) (Variables|/Game/_CardfieldPrototype/TestingPlayground/Filip/Slot/BP_MapManager.BP_MapManager_C|GetMargin (Variables|Default|GetMapManager))) -1.3e+02) (.y (LocalVariables|GetSpawnLocation)) (.z (LocalVariables|GetSpawnLocation)))))))

(fn RecalculateVisibility
  (params (Cards :type Array%20of%20Actor%20Object%20References))
  (bind _mapmanager (Variables|Default|GetMapManager))
  (bind _mapmanager_2 (Variables|Default|GetMapManager))
  (bind _mapmanager_3 (Variables|Default|GetMapManager))
  (bind _height (Variables|/Game/_CardfieldPrototype/TestingPlayground/Filip/Slot/BP_MapManager.BP_MapManager_C|GetHeight _mapmanager_3))
  (for _index (range 0 (- (* (Variables|/Game/_CardfieldPrototype/TestingPlayground/Filip/Slot/BP_MapManager.BP_MapManager_C|GetHeight _mapmanager) (Variables|/Game/_CardfieldPrototype/TestingPlayground/Filip/Slot/BP_MapManager.BP_MapManager_C|GetWidth _mapmanager)) 1))
    (Utilities|Array|SetArrayElem (Variables|Default|GetTargetFade) _index 1.0))
  (for _array_element Cards
    (bind _index_2 (Class|BPItoMapManager|GetSlotIndex(Message) (Variables|Default|GetMapManager) _array_element))
    (LocalVariables|SetSlotIndex _index_2)
    (LocalVariables|SetCardX (/ (LocalVariables|GetSlotIndex) _height))
    (LocalVariables|SetCardY (Math|Integer|%(Integer) (LocalVariables|GetSlotIndex) _height))
    (bind _vision (Class|BPItoCard|GetVision(Message) _array_element))
    (bind _output_get (LocalVariables|SetVision _vision))
    (for _index_3 (range (* _output_get -1) _output_get)
      (LocalVariables|SetDX _index_3)
      (for _index_4 (range (* (LocalVariables|GetVision) -1) (LocalVariables|GetVision))
        (LocalVariables|SetDY _index_4)
        (if (<= (+ (Math|Integer|Absolute(Integer) (LocalVariables|GetDX)) (Math|Integer|Absolute(Integer) (LocalVariables|GetDY))) (LocalVariables|GetVision))
          (LocalVariables|SetSlotX (+ (LocalVariables|GetCardX) (LocalVariables|GetDX)))
          (LocalVariables|SetSlotY (+ (LocalVariables|GetCardY) (LocalVariables|GetDY)))
          (if (Math|Boolean|ANDBoolean (>= (LocalVariables|GetSlotX) 0) (< (LocalVariables|GetSlotX) (Variables|/Game/_CardfieldPrototype/TestingPlayground/Filip/Slot/BP_MapManager.BP_MapManager_C|GetWidth _mapmanager_2)) (>= (LocalVariables|GetSlotY) 0) (< (LocalVariables|GetSlotY) (Variables|/Game/_CardfieldPrototype/TestingPlayground/Filip/Slot/BP_MapManager.BP_MapManager_C|GetHeight _mapmanager_2)))
            (Utilities|Array|SetArrayElem (Variables|Default|GetTargetFade) (+ (* (LocalVariables|GetSlotX) (Variables|/Game/_CardfieldPrototype/TestingPlayground/Filip/Slot/BP_MapManager.BP_MapManager_C|GetHeight (Variables|Default|GetMapManager))) (LocalVariables|GetSlotY)) 0.0))))))
  (for _array_element_2 (Variables|Default|GetBaseVisibility)
    (Utilities|Array|SetArrayElem (Variables|Default|GetTargetFade) _array_element_2 0.0))
  (Actor|Tick|SetActorTickEnabled true)
  (CallFunction|CheckCardsVisibility))

(fn CheckCardsVisibility
  (bind _cards (Class|BPItoGameMode|GetEnemyCards(Message) (Game|GetGameMode)))
  (for _array_element _cards
    (bind _index (Class|BPItoMapManager|GetSlotIndex(Message) (Variables|Default|GetMapManager) _array_element))
    (Rendering|SetActorHiddenInGame _array_element (> (Utilities|Array|Get(acopy) (Variables|Default|GetTargetFade) _index) 0.1)))
  (return))

(fn SetBaseVisibility
  (params (BaseVisibilityIndexes :type Array%20of%20Integers) (AIBaseVisibilityIndexes :type Array%20of%20Integers))
  (Variables|Default|SetBaseVisibility BaseVisibilityIndexes)
  (Variables|Default|SetAIBaseVisibility AIBaseVisibilityIndexes))

(fn GetandCalculateVisibility
  (params (Cards :type Array%20of%20Actor%20Object%20References) (AI%20Base :type Boolean))
  (bind (_width _height) (Class|BPItoMapManager|GetMapSize(Message) (Variables|Default|GetMapManager)))
  (for _index (range 0 (- (* _width _height) 1))
    (Utilities|Array|SetArrayElem (LocalVariables|GetMap) _index false)
    (Utilities|Array|SetArrayElem (LocalVariables|GetBase) _index false)
    (Utilities|Array|SetArrayElem (LocalVariables|GetAllayCards) _index false))
  (for _array_element Cards
    (bind _index_2 (Class|BPItoMapManager|GetSlotIndex(Message) (Variables|Default|GetMapManager) _array_element))
    (LocalVariables|SetSlotIndex _index_2)
    (LocalVariables|SetCardX (/ (LocalVariables|GetSlotIndex) _height))
    (LocalVariables|SetCardY (Math|Integer|%(Integer) (LocalVariables|GetSlotIndex) _height))
    (bind _vision (Class|BPItoCard|GetVision(Message) _array_element))
    (bind _output_get (LocalVariables|SetVision _vision))
    (for _index_3 (range (* _output_get -1) _output_get)
      (LocalVariables|SetDX _index_3)
      (for _index_4 (range (* (LocalVariables|GetVision) -1) (LocalVariables|GetVision))
        (LocalVariables|SetDY _index_4)
        (if (<= (+ (Math|Integer|Absolute(Integer) (LocalVariables|GetDX)) (Math|Integer|Absolute(Integer) (LocalVariables|GetDY))) (LocalVariables|GetVision))
          (LocalVariables|SetSlotX (+ (LocalVariables|GetCardX) (LocalVariables|GetDX)))
          (LocalVariables|SetSlotY (+ (LocalVariables|GetCardY) (LocalVariables|GetDY)))
          (bind (_width_2 _height_2) (Class|BPItoMapManager|GetMapSize(Message) (Variables|Default|GetMapManager)))
          (if (Math|Boolean|ANDBoolean (>= (LocalVariables|GetSlotX) 0) (< (LocalVariables|GetSlotX) _width_2) (>= (LocalVariables|GetSlotY) 0) (< (LocalVariables|GetSlotY) _height_2))
            (Utilities|Array|SetArrayElem (LocalVariables|GetMap) (Default|CordstoIndex (Variables|Default|GetMapManager) (LocalVariables|GetSlotX) (LocalVariables|GetSlotY)) true)
            (Utilities|Array|SetArrayElem (LocalVariables|GetAllayCards) (Default|CordstoIndex (Variables|Default|GetMapManager) (LocalVariables|GetSlotX) (LocalVariables|GetSlotY)) true))))))
  (for _array_element_2 (select AI%20Base (Variables|Default|GetAIBaseVisibility) (Variables|Default|GetBaseVisibility))
    (Utilities|Array|SetArrayElem (LocalVariables|GetMap) _array_element_2 true)
    (Utilities|Array|SetArrayElem (LocalVariables|GetBase) _array_element_2 true))
  (return (LocalVariables|GetMap) (LocalVariables|GetBase) (LocalVariables|GetAllayCards)))