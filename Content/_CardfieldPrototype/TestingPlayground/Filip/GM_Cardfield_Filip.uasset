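; Game mode for Filip's testing playground in the Cardfield prototype that keeps track of the enemy's cards.
; It holds an EnemyCards collection, with an event to add a card, a function to remove one and return the updated collection, and a getter.
; BeginPlay only prints a game-start message, and Tick does nothing.
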(event EventBeginPlay
  (Development|PrintString "GAME START"))

(event EventTick
  (params (DeltaSeconds :type Float%20%28single-precision%29)))

(event EventAddCardtoEnemyCards
  (params (Card :type Actor%20Object%20Reference))
  (Utilities|Array|Add (Variables|Default|GetEnemyCards) Card))

(fn ConstructionScript)

(fn GetEnemyCards
  (return (Variables|Default|GetEnemyCards)))

(fn RemoveCardfromEnemyCards
  (params (Card :type Actor%20Object%20Reference))
  (Utilities|Array|RemoveItem (Variables|Default|GetEnemyCards) Card)
  (return (Variables|Default|GetEnemyCards)))