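; Prototype map manager for a two-player card game that builds the slot grid, marks both players' base rows and spawns four test cards on random slots.
; Slots live in one flat array, whose index math drives neighbor, direction and mask-to-slot queries.
; Movement helpers build speed-limited paths, either along columns by camera yaw or cell by cell under the cursor with backtracking.
; SortedMove attempts a bubble sort of moves by row.
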(event EventBeginPlay
  (CallFunction|InitMap)
  (CallFunction|ConvertMaptoBaseSlots)
  (bind _output_get (Variables|Default|SetTempRandom (.OutItem (Utilities|Array|Random (Variables|Default|GetSlots)))))
  (bind _asbp_slot (Utilities|Casting|CastToBP_Slot _output_get)) ; Prototype == HardRef
  (bind _returnvalue (Game|SpawnActorfromClass "/Game/_CardfieldPrototype/TestingPlayground/Filip/Card/BP_Card.BP_Card_C" (Math|Transform|MakeTransform (Transformation|GetActorLocation _output_get) "0, 0, 0" "1.000000,1.000000,1.000000") "AlwaysSpawn" "MultiplyWithRoot" 0 true _asbp_slot "/Game/_CardfieldPrototype/TestingPlayground/Filip/Card/DA_Card1.DA_Card1" 0))
  (Variables|/Game/_CardfieldPrototype/TestingPlayground/Filip/Slot/BP_Slot.BP_Slot_C|SetCard _asbp_slot _returnvalue)
  (bind _output_get_2 (Variables|Default|SetTempRandom (.OutItem (Utilities|Array|Random (Variables|Default|GetSlots)))))
  (bind _asbp_slot_2 (Utilities|Casting|CastToBP_Slot _output_get_2)) ; Prototype == HardRef
  (bind _returnvalue_2 (Game|SpawnActorfromClass "/Game/_CardfieldPrototype/TestingPlayground/Filip/Card/BP_Card.BP_Card_C" (Math|Transform|MakeTransform (Transformation|GetActorLocation _output_get_2) "0, 0, 0" "1.000000,1.000000,1.000000") "AlwaysSpawn" "MultiplyWithRoot" 0 true _asbp_slot_2 "/Game/_CardfieldPrototype/TestingPlayground/Filip/Card/DA_Card1.DA_Card1" 0))
  (Variables|/Game/_CardfieldPrototype/TestingPlayground/Filip/Slot/BP_Slot.BP_Slot_C|SetCard _asbp_slot_2 _returnvalue_2)
  (bind _output_get_3 (Variables|Default|SetTempRandom (.OutItem (Utilities|Array|Random (Variables|Default|GetSlots)))))
  (bind _asbp_slot_3 (Utilities|Casting|CastToBP_Slot _output_get_3)) ; Prototype == HardRef
  (bind _returnvalue_3 (Game|SpawnActorfromClass "/Game/_CardfieldPrototype/TestingPlayground/Filip/Card/BP_Card.BP_Card_C" (Math|Transform|MakeTransform (Transformation|GetActorLocation _output_get_3) "0, 0, 0" "1.000000,1.000000,1.000000") "AlwaysSpawn" "MultiplyWithRoot" 0 false _asbp_slot_3 "/Game/_CardfieldPrototype/TestingPlayground/Filip/Card/DA_Card2.DA_Card2" 0))
  (Variables|/Game/_CardfieldPrototype/TestingPlayground/Filip/Slot/BP_Slot.BP_Slot_C|SetCard _asbp_slot_3 _returnvalue_3)
  (bind _output_get_4 (Variables|Default|SetTempRandom (.OutItem (Utilities|Array|Random (Variables|Default|GetSlots)))))
  (bind _asbp_slot_4 (Utilities|Casting|CastToBP_Slot _output_get_4)) ; Prototype == HardRef
  (bind _returnvalue_4 (Game|SpawnActorfromClass "/Game/_CardfieldPrototype/TestingPlayground/Filip/Card/BP_Card.BP_Card_C" (Math|Transform|MakeTransform (Transformation|GetActorLocation _output_get_4) "0, 0, 0" "1.000000,1.000000,1.000000") "AlwaysSpawn" "MultiplyWithRoot" 0 false _asbp_slot_4 "/Game/_CardfieldPrototype/TestingPlayground/Filip/Card/DA_Card2.DA_Card2" 0))
  (Variables|/Game/_CardfieldPrototype/TestingPlayground/Filip/Slot/BP_Slot.BP_Slot_C|SetCard _asbp_slot_4 _returnvalue_4))

(fn ConstructionScript)

(fn InitMap
  (for _index (range 1 (Variables|Default|GetWidth))
    (LocalVariables|SetSpawnLocation (+ (Transformation|GetActorLocation) (* (Math|Vector|MakeVector 0.0 (+ -1e+02 (Variables|Default|GetMargin)) 0.0) _index)))
    (for _index_2 (range 1 (Variables|Default|GetHeight))
      (bind _returnvalue (Game|SpawnActorfromClass "/Game/_CardfieldPrototype/TestingPlayground/Filip/Slot/BP_Slot.BP_Slot_C" (Math|Transform|MakeTransform (Math|Vector|MakeVector (+ (+ (.x (LocalVariables|GetSpawnLocation)) (Variables|Default|GetMargin)) -1.3e+02) (.y (LocalVariables|GetSpawnLocation)) (.z (LocalVariables|GetSpawnLocation))) "0, 0, 0" "1.000000,1.000000,1.000000") "AlwaysSpawn" "MultiplyWithRoot" 0 0))
      (LocalVariables|SetSpawnLocation (Transformation|GetActorLocation _returnvalue))
      (Utilities|Array|Add (Variables|Default|GetSlots) _returnvalue))))

(fn GetColumnPath
  (params (Slot :type Actor%20Object%20Reference) (SelectedSlot :type Actor%20Object%20Reference))
  (bind _slots (Variables|Default|GetSlots))
  (bind _finalreturn (LocalVariables|GetFinalReturn))
  (bind _returnvalue (Utilities|Array|FindItem _slots SelectedSlot))
  (bind _returnvalue_2 (Utilities|Array|LastIndex _finalreturn))
  (bind _output (Utilities|Array|Get(acopy) _finalreturn _returnvalue_2))
  (bind _asbp_slot (Utilities|Casting|CastToBP_Slot Slot))
  ;[0.15 0.15 0.15 0.5] current
  (if (Default|IsBaseSlot _asbp_slot)
    (LocalVariables|SetBaseSlot Slot))
  (LocalVariables|SetStartX (/ _returnvalue (Variables|Default|GetHeight)))
  (LocalVariables|SetStartY (Math|Integer|%(Integer) _returnvalue (Variables|Default|GetHeight)))
  (LocalVariables|SetEndY (Math|Integer|%(Integer) (Utilities|Array|FindItem (Variables|Default|GetSlots) Slot) (Variables|Default|GetHeight)))
  (LocalVariables|SetMaxY (Math|Integer|Absolute(Integer) (- (LocalVariables|GetEndY) (LocalVariables|GetStartY))))
  (bind _asbp_slot_2 (Utilities|Casting|CastToBP_Slot SelectedSlot)) ; Prototype
  (bind _asbp_card (Utilities|Casting|CastToBP_Card (Variables|/Game/_CardfieldPrototype/TestingPlayground/Filip/Slot/BP_Slot.BP_Slot_C|GetCard _asbp_slot_2)))
  (LocalVariables|SetStepToDo (Math|Integer|Min(Integer) (LocalVariables|GetMaxY) (Variables|/Game/_CardfieldPrototype/TestingPlayground/Filip/Card/PDA_CardStats.PDA_CardStats_C|GetSpeed (Variables|/Game/_CardfieldPrototype/TestingPlayground/Filip/Card/BP_Card.BP_Card_C|GetStats _asbp_card))))
  (if (== (LocalVariables|GetStartY) (LocalVariables|GetEndY))
    (return (LocalVariables|GetFinalReturn))
    (else
      (LocalVariables|SetStep (Math|Integer|SelectInt 1 -1 (> (Math|Float|Sign(Float) (.yaw (Camera|GetCameraRotation (Variables|/Script/Engine.PlayerController|GetPlayerCameraManager (Game|GetPlayerController 0))))) 0.0)))
      ;[0.15 0.15 0.15 0.5] XD prototype
      (bind _asbp_slot_3 (Utilities|Casting|CastToBP_Slot SelectedSlot))
      (bind _asbp_card_2 (Utilities|Casting|CastToBP_Card (Variables|/Game/_CardfieldPrototype/TestingPlayground/Filip/Slot/BP_Slot.BP_Slot_C|GetCard _asbp_slot_3)))
      (bind _index (Utilities|FlowControl|ForLoopwithBreak 1 (LocalVariables|GetStepToDo) :!label _label)
        (:LoopBody
          (bind _output_get (LocalVariables|SetCurrentY (+ (* _index (LocalVariables|GetStep)) (LocalVariables|GetStartY))))
          (if (or (< _output_get 0) (> _output_get (- (Variables|Default|GetHeight) 1)))
            (Development|PrintString "Something wrong" true true "(R=1.000000,G=0.000000,B=0.001830,A=1.000000)" 2.0 "IDX" :!label _label_2)
            (goto _label Break)
            (elif (and (> (LocalVariables|GetStep) 0) (> (LocalVariables|GetCurrentY) (LocalVariables|GetEndY)))
              (goto _label_2)
              (elif (and (< (LocalVariables|GetStep) 0) (< (LocalVariables|GetCurrentY) (LocalVariables|GetEndY)))
                (goto _label_2)
                (elif (Utilities|Array|IsValidIndex (Variables|Default|GetSlots) (+ (LocalVariables|GetCurrentY) (* (LocalVariables|GetStartX) (Variables|Default|GetHeight))))
                  (Utilities|Array|Add (LocalVariables|GetFinalReturn) (Utilities|Array|Get(acopy) (Variables|Default|GetSlots) (+ (LocalVariables|GetCurrentY) (* (LocalVariables|GetStartX) (Variables|Default|GetHeight)))))
                  (else
                    (Development|PrintString "INDEX IS NOT VALID" true true "(R=1.000000,G=0.000000,B=0.001830,A=1.000000)" 2.0 "IDX")
                    (return (Utilities|Array|MakeArray))))))))
        (:Completed
          (Utilities|Array|RemoveItem (LocalVariables|GetFinalReturn) (LocalVariables|GetBaseSlot))
          (bind _asbp_slot_4 (Utilities|Casting|CastToBP_Slot _output))
          ;[0.15 0.15 0.15 0.5] current
          (if (Default|IsBaseSlot _asbp_slot_4)
            (Utilities|Array|RemoveItem (LocalVariables|GetFinalReturn) _output))
          (return (LocalVariables|GetFinalReturn)))))))

(fn SortedMove
  (params (Map :type Map%20of%20BP%20Card%20Object%20References%20to%20Structs))
  (bind _returnvalue (Utilities|Map|Length Map))
  (bind _returnvalue_2 (- _returnvalue 1))
  (bind _values (Utilities|Map|Values Map))
  (LocalVariables|SetValues _values)
  (for _index (range 0 _returnvalue_2)
    (bind _index_2 (Utilities|FlowControl|ForLoopwithBreak 0 (Utilities|Operators|Subtract _returnvalue_2 _index 1) :!label _label)
      (:LoopBody
        (Variables|/Game/_CardfieldPrototype/TestingPlayground/Filip/Card/BP_Card.BP_Card_C|GetbPlayerOne (.card (Utilities|Array|Get(acopy) (LocalVariables|GetValues) _index_2))
          (:then
            (if (< (Math|Integer|%(Integer) (Utilities|Array|FindItem (Variables|Default|GetSlots) (Variables|/Game/_CardfieldPrototype/TestingPlayground/Filip/Card/BP_Card.BP_Card_C|GetmySlot (.card (Utilities|Array|Get(acopy) (LocalVariables|GetValues) _index_2)))) (Variables|Default|GetHeight)) (Math|Integer|%(Integer) (Utilities|Array|FindItem (Variables|Default|GetSlots) (Variables|/Game/_CardfieldPrototype/TestingPlayground/Filip/Card/BP_Card.BP_Card_C|GetmySlot (.card (Utilities|Array|Get(acopy) (LocalVariables|GetValues) (+ _index_2 1))))) (Variables|Default|GetHeight)))
              (Utilities|Array|Swap (LocalVariables|GetValues) _index_2 (+ _index_2 1))
              (goto _label Break)))
          (:else
            (if (> (Math|Integer|%(Integer) (Utilities|Array|FindItem (Variables|Default|GetSlots) (Variables|/Game/_CardfieldPrototype/TestingPlayground/Filip/Card/BP_Card.BP_Card_C|GetmySlot (.card (Utilities|Array|Get(acopy) (LocalVariables|GetValues) _index_2)))) (Variables|Default|GetHeight)) (Math|Integer|%(Integer) (Utilities|Array|FindItem (Variables|Default|GetSlots) (Variables|/Game/_CardfieldPrototype/TestingPlayground/Filip/Card/BP_Card.BP_Card_C|GetmySlot (.card (Utilities|Array|Get(acopy) (LocalVariables|GetValues) (+ _index_2 1))))) (Variables|Default|GetHeight)))
              (Utilities|Array|Swap (LocalVariables|GetValues) _index_2 (+ _index_2 1))))))
      (:Completed
        (for _array_element (LocalVariables|GetValues)
          (Utilities|Map|Add (LocalVariables|GetMapOutFinal) (.card _array_element) (Utilities|Struct|MakeS_Lines (.card _array_element) (.array _array_element))))
        (return (LocalVariables|GetMapOutFinal))))))

(fn ConvertMaptoBaseSlots
  (bind _height (Variables|Default|GetHeight))
  (for (_array_element _array_index) (Variables|Default|GetSlots)
    (if (== (Math|Integer|%(Integer) _array_index _height) 0)
      (bind _asbp_slot (Utilities|Casting|CastToBP_Slot _array_element))
      (Variables|/Game/_CardfieldPrototype/TestingPlayground/Filip/Slot/BP_Slot.BP_Slot_C|SetPlayerOneSlot_Base _asbp_slot true)
      ;[0.15 0.15 0.15 0.5] current
      (Variables|/Game/_CardfieldPrototype/TestingPlayground/Filip/Slot/BP_Slot.BP_Slot_C|SetSlotType _asbp_slot "NewEnumerator5")
      (Default|BaseMaterial _asbp_slot)
      (elif (== (Math|Integer|%(Integer) _array_index _height) (- _height 1))
        (bind _asbp_slot_2 (Utilities|Casting|CastToBP_Slot _array_element))
        (Variables|/Game/_CardfieldPrototype/TestingPlayground/Filip/Slot/BP_Slot.BP_Slot_C|SetPlayerOneSlot_Base _asbp_slot_2 false)
        ;[0.15 0.15 0.15 0.5] current
        (Variables|/Game/_CardfieldPrototype/TestingPlayground/Filip/Slot/BP_Slot.BP_Slot_C|SetSlotType _asbp_slot_2 "NewEnumerator5")
        (Default|BaseMaterial _asbp_slot_2)))))

(fn ConvertMasktoMap
  (params (Slot :type Actor%20Object%20Reference) (Mask :type Array%20of%20Int%20Point%20Structures))
  (bind _slots (Variables|Default|GetSlots))
  (bind _height (Variables|Default|GetHeight))
  (bind _returnvalue (Utilities|Array|FindItem _slots Slot))
  (LocalVariables|SetStartX (/ _returnvalue _height))
  (LocalVariables|SetStartY (Math|Integer|%(Integer) _returnvalue _height))
  (for _array_element Mask
    (LocalVariables|SetTargetX (+ (.X (Utilities|Struct|BreakIntPoint _array_element)) (LocalVariables|GetStartX)))
    (LocalVariables|SetTargetY (+ (.Y (Utilities|Struct|BreakIntPoint _array_element)) (LocalVariables|GetStartY)))
    (if (and (>= (LocalVariables|GetTargetX) 0) (< (LocalVariables|GetTargetX) (Variables|Default|GetWidth)))
      (if (and (>= (LocalVariables|GetTargetY) 0) (< (LocalVariables|GetTargetY) (Variables|Default|GetHeight)))
        (if (Utilities|Array|IsValidIndex (Variables|Default|GetSlots) (+ (* (LocalVariables|GetTargetX) (Variables|Default|GetHeight)) (LocalVariables|GetTargetY)))
          (Utilities|Array|Add (LocalVariables|GetResults) (Utilities|Array|Get(acopy) (Variables|Default|GetSlots) (+ (* (LocalVariables|GetTargetX) (Variables|Default|GetHeight)) (LocalVariables|GetTargetY))))))))
  (return (LocalVariables|GetResults)))

(fn DoPathifPossible
  (params (NewSlot :type Actor%20Object%20Reference) (CurrentPath :type Array%20of%20Actor%20Object%20References))
  (LocalVariables|SetResultPath CurrentPath)
  (if (Utilities|Array|IsEmpty CurrentPath) ; Gdyby jakimś cudem \nusunięto punkt startowy.
    (Utilities|Array|Insert (LocalVariables|GetResultPath) NewSlot))
  (Utilities|IsValid NewSlot ; Czy myszka wskazuje na slot?
    (:Is%20Valid
      (if (== NewSlot (Utilities|Array|Get(acopy) (LocalVariables|GetResultPath) (Utilities|Array|LastIndex (LocalVariables|GetResultPath)))) ; Czy wskazany element to\nostatni element w Path?\nGracz jeszcze nie zdążył\nprzesunąć myszki na inny\nslot.
        _
        (else
          (if (CallFunction|IsCardinalNeigbor NewSlot (Utilities|Array|Get(acopy) (LocalVariables|GetResultPath) (Utilities|Array|LastIndex (LocalVariables|GetResultPath)))) ; Czy nowy slot jest sąsiadem\nostatniego slota w Path?
            (if (Utilities|Array|ContainsItem (LocalVariables|GetResultPath) NewSlot) ; Rozgałęzienie decydujące,\nczy możemy normalnie dodać,\nczy może być konflikt.
              (if (== NewSlot (Utilities|Array|Get(acopy) (LocalVariables|GetResultPath) (- (Utilities|Array|Length (LocalVariables|GetResultPath)) 2))) ; Jeśli to przedostatni element,\npo prostu skróć ścieżkę o jeden.
                (Utilities|Array|RemoveIndex (LocalVariables|GetResultPath) (Utilities|Array|LastIndex (LocalVariables|GetResultPath)))
                (return (LocalVariables|GetResultPath))
                (else
                  _))
              (else
                (bind _asbp_slot (Utilities|Casting|CastToBP_Slot (Utilities|Array|Get(acopy) (LocalVariables|GetResultPath))))
                (bind _asbp_card (Utilities|Casting|CastToBP_Card (Variables|/Game/_CardfieldPrototype/TestingPlayground/Filip/Slot/BP_Slot.BP_Slot_C|GetCard _asbp_slot)))
                (if (<= (Utilities|Array|Length (LocalVariables|GetResultPath)) (Variables|/Game/_CardfieldPrototype/TestingPlayground/Filip/Card/BPC_StatsComponent.BPC_StatsComponent_C|GetSpeedLeft (Variables|/Game/_CardfieldPrototype/TestingPlayground/Filip/Card/BP_Card.BP_Card_C|GetBPC_StatsComponent _asbp_card)))
                  ;[0.15 0.15 0.15 0.5] current
                  (if (Default|IsBaseSlot _asbp_slot)
                    (if (== (Variables|/Game/_CardfieldPrototype/TestingPlayground/Filip/Slot/BP_Slot.BP_Slot_C|GetPlayerOneSlot_Base _asbp_slot) (Variables|/Game/_CardfieldPrototype/TestingPlayground/Filip/Card/BP_Card.BP_Card_C|GetbPlayerOne _asbp_card))
                      _
                      (else
                        (return (LocalVariables|GetResultPath)))))
                  (Utilities|Array|Add (LocalVariables|GetResultPath) NewSlot)
                  (return (LocalVariables|GetResultPath))
                  (else
                    (return (LocalVariables|GetResultPath))))))
            (elif (Utilities|Array|ContainsItem (LocalVariables|GetResultPath) NewSlot) ; Sprawdzenie, czy gracz może chciał\nszybko zresetować ścieżkę.
              _
              (else
                (return (LocalVariables|GetResultPath)))))
          (bind _output_get (LocalVariables|SetConflictIndex (Utilities|Array|FindItem (LocalVariables|GetResultPath) NewSlot)))
          (while (Utilities|Array|IsValidIndex (LocalVariables|GetResultPath) _output_get) ; Pojawiło się przecięcie\ni trzeba zresetować Path\ndo miejsca przecięcia.
            (Utilities|Array|RemoveIndex (LocalVariables|GetResultPath) (LocalVariables|GetConflictIndex)))
          (Utilities|Array|Add (LocalVariables|GetResultPath) NewSlot)
          (return (LocalVariables|GetResultPath)))))
    (:Is%20Not%20Valid
      _))
  (return (LocalVariables|GetResultPath)))

(fn IsCardinalNeigbor
  (params (SlotA :type Actor%20Object%20Reference) (SlotB :type Actor%20Object%20Reference))
  (bind _slots (Variables|Default|GetSlots))
  (bind _height (Variables|Default|GetHeight))
  (bind _slots_2 (Variables|Default|GetSlots))
  (bind _height_2 (Variables|Default|GetHeight))
  (bind _returnvalue (Utilities|Array|FindItem _slots SlotB))
  (bind _returnvalue_2 (Utilities|Array|FindItem _slots_2 SlotA))
  (return (== (+ (Math|Integer|Absolute(Integer) (- (/ _returnvalue_2 _height_2) (/ _returnvalue _height))) (Math|Integer|Absolute(Integer) (- (Math|Integer|%(Integer) _returnvalue_2 _height_2) (Math|Integer|%(Integer) _returnvalue _height)))) 1)))

(fn GetDir
  (params (Slot%201 :type Actor%20Object%20Reference) (Slot%202 :type Actor%20Object%20Reference))
  (bind _slots (Variables|Default|GetSlots))
  (bind _slots_2 (Variables|Default|GetSlots))
  (bind _height (Variables|Default|GetHeight))
  (bind _height_2 (Variables|Default|GetHeight))
  (bind _returnvalue (Utilities|Array|FindItem _slots Slot%202))
  (bind _returnvalue_2 (Utilities|Array|FindItem _slots_2 Slot%201))
  (LocalVariables|SetA.X (/ _returnvalue_2 _height_2))
  (LocalVariables|SetA.Y (Math|Integer|%(Integer) _returnvalue_2 _height_2))
  (LocalVariables|SetB.X (/ _returnvalue _height))
  (LocalVariables|SetB.Y (Math|Integer|%(Integer) _returnvalue _height))
  (if (== (LocalVariables|GetB.Y) (+ (LocalVariables|GetA.Y) 1))
    (return "Up")
    (elif (== (LocalVariables|GetB.X) (+ (LocalVariables|GetA.X) 1))
      (return "Right")
      (elif (== (LocalVariables|GetB.Y) (- (LocalVariables|GetA.Y) 1))
        (return "Down")
        (elif (== (LocalVariables|GetB.X) (- (LocalVariables|GetA.X) 1))
          (return "Left")
          (elif (not (and (== (LocalVariables|GetA.X) (LocalVariables|GetB.X)) (== (LocalVariables|GetA.Y) (LocalVariables|GetB.Y))))
            (Development|PrintText (Utilities|Text|FormatText "ERROR GET_DIR: ({X1}, {Y1}) ({X2}, {Y2})" (LocalVariables|GetA.X) (LocalVariables|GetA.Y) (LocalVariables|GetB.X) (LocalVariables|GetB.Y)) true true "(R=1.000000,G=0.000000,B=0.001830,A=1.000000)" 2.0 "testerr")))))))