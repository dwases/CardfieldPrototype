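; BP_Slot is a card battlefield slot actor that spawns and tracks a BP_Card, with a slot type that selects its material.
; On the controller's player-change event, occupied slots run type effects: healing, damage, or resource and excavation handling that reverts the slot to Default.
; Custom primitive data on its planes drives base, attack-highlight and arrow visuals.
; Persistent effects and general slot logic are empty stubs, and Printer only prints debug text.
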(event Custom|Default%20Material
  (Rendering|Material|SetCustomPrimitiveDataFloat (Variables|Default|GetPlane) 0 0.0)
  (Rendering|Material|SetCustomPrimitiveDataFloat (Variables|Default|GetArrowPlane) 5 0.0))

(event Custom|Line%20Material
  (params (Rotation :type Float%20%28double-precision%29) (Turn :type Boolean) (Mirror :type Boolean) (Visible :type Boolean))
  (bind _arrowplane (Variables|Default|GetArrowPlane))
  (Rendering|Material|SetCustomPrimitiveDataFloat _arrowplane 0 1.0)
  (Rendering|Material|SetCustomPrimitiveDataFloat _arrowplane 1 Rotation)
  (Rendering|Material|SetCustomPrimitiveDataFloat _arrowplane 3 (Math|Float|SelectFloat 1.0 0.0 Turn))
  (Rendering|Material|SetCustomPrimitiveDataFloat _arrowplane 4 (Math|Float|SelectFloat 1.0 0.0 Mirror))
  (Rendering|Material|SetCustomPrimitiveDataFloat _arrowplane 5 (Math|Float|SelectFloat 1.0 0.0 Visible)))

(event Custom|Base%20Material
  (Rendering|Material|SetCustomPrimitiveDataFloat (Variables|Default|GetPlane) 2 1.0))

(event Custom|SpawnOnDrop
  (params (PlayerOne :type Boolean) (Stats :type PDA%20Card%20Stats%20Object%20Reference))
  (bind _self self)
  (bind _returnvalue (Game|SpawnActorfromClass "/Game/_CardfieldPrototype/TestingPlayground/Filip/Card/BP_Card.BP_Card_C" (Transformation|GetActorTransform _self) "AlwaysSpawn" "MultiplyWithRoot" 0 PlayerOne _self Stats 0))
  (Variables|Default|SetCard _returnvalue)
  (bind _aspc_controller_filip (Utilities|Casting|CastToPC_Controller_Filip (Game|GetPlayerController 0)))
  (Variables|/Game/_CardfieldPrototype/TestingPlayground/Filip/PC_Controller_Filip.PC_Controller_Filip_C|GetPlayerOneTurn _aspc_controller_filip
    (:then)
    (:else
      (Default|RotateWidget _returnvalue))))

(event Custom|Attack%20Material%20ON
  (params (Pulse :type Boolean))
  (bind _aspc_controller_filip (Utilities|Casting|CastToPC_Controller_Filip (Game|GetPlayerController 0)))
  (Rendering|Material|SetCustomPrimitiveDataFloat (Variables|Default|GetTranslucentPlane) 1 (Math|Float|SelectFloat 0.25 0.75 (Variables|/Game/_CardfieldPrototype/TestingPlayground/Filip/PC_Controller_Filip.PC_Controller_Filip_C|GetPlayerOneTurn _aspc_controller_filip)))
  (Rendering|Material|SetCustomPrimitiveDataFloat (Variables|Default|GetTranslucentPlane) 0 1.0)
  (Rendering|Material|SetCustomPrimitiveDataFloat (Variables|Default|GetTranslucentPlane) 2 (Math|Float|SelectFloat 1.0 0.0 Pulse))
  (Variables|Default|SetAttackable true))

(event Custom|Attack%20Material%20OFF
  (Rendering|Material|SetCustomPrimitiveDataFloat (Variables|Default|GetTranslucentPlane) 0 0.0)
  (Variables|Default|SetAttackable false)
  (Rendering|Material|SetCustomPrimitiveDataFloat (Variables|Default|GetTranslucentPlane) 2 0.0))

(event Custom|SwitchSlotType
  (params (NewSlotType :type E_SlotType%20Enum :default "NewEnumerator0"))
  (Variables|Default|SetSlotType NewSlotType)
  (CallFunction|RefreshSlotVisuals))

(event Custom|CallActivatePerTurnSlotEffect
  (CallFunction|ActivatePerTurnSlotEffect))

(event Custom|ExecSlotLogic
  ;[0.15 0.15 0.15 0.5] WIP
)

(event EventBeginPlay
  (bind _aspc_controller_filip (Utilities|Casting|CastToPC_Controller_Filip (Game|GetPlayerController 0)))
  (EventDispatchers|BindEventtoOnPlayerChange _aspc_controller_filip (delegate Custom|CallActivatePerTurnSlotEffect))
  ;[0.15 0.15 0.15 0.5] for future features
  (CallFunction|ActivatePersistentSlotEffect))

(event Collision|EventActorBeginOverlap
  (params (OtherActor :type Actor%20Object%20Reference)))

(event EventTick
  (params (DeltaSeconds :type Float%20%28single-precision%29)))

(event EventSetDefaultMaterial
  (Rendering|Material|SetCustomPrimitiveDataFloat (Variables|Default|GetPlane) 0 0.0)
  (Rendering|Material|SetCustomPrimitiveDataFloat (Variables|Default|GetArrowPlane) 5 0.0))

(event EventAssignCard
  (params (Card :type Actor%20Object%20Reference))
  (Variables|Default|SetCard Card))

(event EventUnassignCard
  (Variables|Default|SetCard 0))

(fn ConstructionScript)

(fn IsBaseSlot
  (return (Utilities|Enum|Equal(Enum) (Variables|Default|GetSlotType) "NewEnumerator5")))

(fn RefreshSlotVisuals
  (switch Utilities|FlowControl|Switch|SwitchonE_SlotType (Variables|Default|GetSlotType)
    (:NewEnumerator7
      (Rendering|Material|SetMaterial (Variables|Default|GetPlane) 0 "/Game/_CardfieldPrototype/TestingPlayground/Filip/HUD/BattleResourceTextures/M_printer.M_printer"))
    (:NewEnumerator2
      ;[0.15 0.15 0.15 0.5] unused- legacy- incompatible with GDD apparently
      (Rendering|Material|SetMaterial (Variables|Default|GetPlane) 0 "/Game/_CardfieldPrototype/TestingPlayground/Filip/HUD/BattleResourceTextures/M_Materials.M_Materials"))
    (:NewEnumerator3
      (Rendering|Material|SetMaterial (Variables|Default|GetPlane) 0 "/Game/_CardfieldPrototype/TestingPlayground/Filip/HUD/BattleResourceTextures/M_Energy.M_Energy"))
    (:NewEnumerator4
      (Rendering|Material|SetMaterial (Variables|Default|GetPlane) 0 "/Game/_CardfieldPrototype/TestingPlayground/Filip/HUD/BattleResourceTextures/M_Minerals.M_Minerals"))
    (:NewEnumerator8
      (Rendering|Material|SetMaterial (Variables|Default|GetPlane) 0 "/Engine/EngineDebugMaterials/BlackUnlitMaterial.BlackUnlitMaterial"))
    (:NewEnumerator9
      (Rendering|Material|SetMaterial (Variables|Default|GetPlane) 0 "/Game/_CardfieldPrototype/TestingPlayground/Filip/HUD/BattleResourceTextures/M_excavation_slot.M_excavation_slot"))
    (:NewEnumerator10
      (Rendering|Material|SetMaterial (Variables|Default|GetPlane) 0 "/Niagara/DefaultAssets/GeometryCache/M_DefaultGeometryCacheMaterial_Green.M_DefaultGeometryCacheMaterial_Green"))
    (:NewEnumerator11
      (Rendering|Material|SetMaterial (Variables|Default|GetPlane) 0 "/AnimationSharing/AnimSharingRed.AnimSharingRed"))
    (:NewEnumerator12
      (Rendering|Material|SetMaterial (Variables|Default|GetPlane) 0 "/Game/_CardfieldPrototype/TestingPlayground/Filip/HUD/BattleResourceTextures/M_rifle.M_rifle"))
    (:NewEnumerator13
      (Rendering|Material|SetMaterial (Variables|Default|GetPlane) 0 "/Game/StarterContent/Props/Materials/M_Rock.M_Rock"))))

(fn ActivatePerTurnSlotEffect
  (Utilities|IsValid (Variables|Default|GetCard)
    (:Is%20Valid
      (switch Utilities|FlowControl|Switch|SwitchonE_SlotType (Variables|Default|GetSlotType)
        (:NewEnumerator7
          ;[0.15 0.15 0.15 0.5] for debug
          (Utilities|Casting|CastToBP_Card (Variables|Default|GetCard))
          (Development|PrintString "slot typu printer został aktywowany, bo zaczela sie tura i stoi na niej jednostka" true true "(R=0.000000,G=0.660000,B=1.000000,A=1.000000)" 5.0 "printer field"))
        (:NewEnumerator1)
        (:NewEnumerator2
          (bind _aspc_controller_filip (Utilities|Casting|CastToPC_Controller_Filip (Game|GetPlayerController 0) :!label _label))
          (Utilities|Struct|SetmembersinS_Resources (Variables|/Game/_CardfieldPrototype/TestingPlayground/Filip/PC_Controller_Filip.PC_Controller_Filip_C|GetResources _aspc_controller_filip) (Utilities|Struct|BreakS_Resources (Variables|/Game/_CardfieldPrototype/TestingPlayground/Filip/PC_Controller_Filip.PC_Controller_Filip_C|GetResources _aspc_controller_filip)))
          (CallFunction|SwitchSlotType "NewEnumerator0" :!label _label_2))
        (:NewEnumerator3
          (bind _aspc_controller_filip_2 (Utilities|Casting|CastToPC_Controller_Filip (Game|GetPlayerController 0) :!label _label_3))
          (Utilities|Struct|SetmembersinS_Resources (Variables|/Game/_CardfieldPrototype/TestingPlayground/Filip/PC_Controller_Filip.PC_Controller_Filip_C|GetResources _aspc_controller_filip_2) (Utilities|Struct|BreakS_Resources (Variables|/Game/_CardfieldPrototype/TestingPlayground/Filip/PC_Controller_Filip.PC_Controller_Filip_C|GetResources _aspc_controller_filip_2)))
          (goto _label_2))
        (:NewEnumerator4
          (bind _aspc_controller_filip_3 (Utilities|Casting|CastToPC_Controller_Filip (Game|GetPlayerController 0) :!label _label_4))
          (Utilities|Struct|SetmembersinS_Resources (Variables|/Game/_CardfieldPrototype/TestingPlayground/Filip/PC_Controller_Filip.PC_Controller_Filip_C|GetResources _aspc_controller_filip_3) (Utilities|Struct|BreakS_Resources (Variables|/Game/_CardfieldPrototype/TestingPlayground/Filip/PC_Controller_Filip.PC_Controller_Filip_C|GetResources _aspc_controller_filip_3)))
          (goto _label_2))
        (:NewEnumerator9
          (switch int (Math|Random|RandomInteger 2)
            (:0
              (goto _label))
            (:1
              (goto _label_3))
            (:2
              (goto _label_4))))
        (:NewEnumerator10
          (bind _asbp_card (Utilities|Casting|CastToBP_Card (Variables|Default|GetCard)))
          (Default|TakeDamage _asbp_card -1))
        (:NewEnumerator11
          (bind _asbp_card_2 (Utilities|Casting|CastToBP_Card (Variables|Default|GetCard)))
          (Default|TakeDamage _asbp_card_2 1))
        (:NewEnumerator12)
        (:NewEnumerator13)))))

(fn ActivatePersistentSlotEffect
  (switch Utilities|FlowControl|Switch|SwitchonE_SlotType (Variables|Default|GetSlotType)))

(fn GetAssignedCard
  (return (Variables|Default|GetCard)))

(fn IsCardAssigned
  (return (Utilities|IsValid (Variables|Default|GetCard))))