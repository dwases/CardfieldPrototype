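; BPC_StatsComponent is a component in the Cardfield prototype that stores a card's gameplay stats, from combat values and movement speed to resources and vision.
; InitStats copies a Stats struct into the component's variables and sets the remaining speed to full.
; TakeDamage subtracts the raw value from Health without using Defense or clamping, then returns the new Health.
; RestoreSpeed refills the remaining speed.
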(event Custom|InitStats
  (params (Stats :type PDA%20Card%20Stats%20Object%20Reference))
  (Variables|Default|SetHealth (Variables|/Game/_CardfieldPrototype/TestingPlayground/Filip/Card/PDA_CardStats.PDA_CardStats_C|GetHealth Stats))
  (Variables|Default|SetAttack (Variables|/Game/_CardfieldPrototype/TestingPlayground/Filip/Card/PDA_CardStats.PDA_CardStats_C|GetAttack Stats))
  (Variables|Default|SetDefense (Variables|/Game/_CardfieldPrototype/TestingPlayground/Filip/Card/PDA_CardStats.PDA_CardStats_C|GetDefense Stats))
  (Variables|Default|SetSpeed (Variables|/Game/_CardfieldPrototype/TestingPlayground/Filip/Card/PDA_CardStats.PDA_CardStats_C|GetSpeed Stats))
  (Variables|Default|SetMaterials (Variables|/Game/_CardfieldPrototype/TestingPlayground/Filip/Card/PDA_CardStats.PDA_CardStats_C|GetMaterials Stats))
  (Variables|Default|SetMinerals (Variables|/Game/_CardfieldPrototype/TestingPlayground/Filip/Card/PDA_CardStats.PDA_CardStats_C|GetMinerals Stats))
  (Variables|Default|SetEnergy (Variables|/Game/_CardfieldPrototype/TestingPlayground/Filip/Card/PDA_CardStats.PDA_CardStats_C|GetEnergy Stats))
  (Variables|Default|SetSpeedLeft (Variables|Default|GetSpeed))
  (Variables|Default|SetVision (Variables|/Game/_CardfieldPrototype/TestingPlayground/Filip/Card/PDA_CardStats.PDA_CardStats_C|GetVision Stats)))

(fn TakeDamage
  (params (Value :type Integer))
  (bind _output_get (Variables|Default|SetHealth (- (Variables|Default|GetHealth) Value)))
  (return _output_get))

(fn RestoreSpeed
  (Variables|Default|SetSpeedLeft (Variables|Default|GetSpeed)))