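; Card actor for a slot-based board, with a stats widget, grid attack mask, movement and damage that destroys it at zero.
; Delayed hover enlarges the widget through a gated Tick interpolation, coordinated with PC_Controller_Filip's state; unhover or click shrinks it.
; Move recursively follows a slot path with a timeline, spending speed per step and stopping at occupied slots.
; BPCStatsComponent holds stats; BeginPlay also binds to the controller's player-change event.
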(event Custom|Move
  (params (Path :type Array%20of%20Actor%20Object%20References))
  (bind _output_get (Variables|Default|SetPath Path))
  (if (Utilities|Array|IsEmpty _output_get)
    (bind _aspc_controller_filip (Utilities|Casting|CastToPC_Controller_Filip (Game|GetPlayerController 0)))
    (Default|SetControllerState _aspc_controller_filip "NewEnumerator0")
    (else
      (bind _asbp_slot (Utilities|Casting|CastToBP_Slot (Utilities|Array|Get(acopy) (Variables|Default|GetPath))))
      (Utilities|IsValid (Variables|/Game/_CardfieldPrototype/TestingPlayground/Filip/Slot/BP_Slot.BP_Slot_C|GetCard _asbp_slot)
        (:Is%20Valid
          (for _array_element (Variables|Default|GetPath)
            (bind _asbp_slot_2 (Utilities|Casting|CastToBP_Slot _array_element))
            (Default|DefaultMaterial _asbp_slot_2))
          (Utilities|Array|Clear (Variables|Default|GetPath))
          (CallFunction|Move (Variables|Default|GetPath)))
        (:Is%20Not%20Valid
          (Variables|/Game/_CardfieldPrototype/TestingPlayground/Filip/Slot/BP_Slot.BP_Slot_C|SetCard (Variables|Default|GetmySlot) 0)
          (bind _output_get_2 (Variables|Default|SetmySlot _asbp_slot))
          (Variables|/Game/_CardfieldPrototype/TestingPlayground/Filip/Slot/BP_Slot.BP_Slot_C|SetCard _output_get_2 self)
          (Default|DefaultMaterial _output_get_2)
          (Components|Timeline|SetPlayRate (Variables|Default|GetMoveTimeline) 4.0)
          (bind _alpha (Timeline|MoveTimeline PlayFromStart)
            (:Update
              (Transformation|SetActorLocation (Math|Vector|Lerp(Vector) (Transformation|GetActorLocation) (Transformation|GetActorLocation (Variables|Default|GetmySlot)) _alpha) false false))
            (:Finished
              (Utilities|Array|RemoveIndex (Variables|Default|GetPath))
              (Math|Integer|DecrementInt (Variables|/Game/_CardfieldPrototype/TestingPlayground/Filip/Card/BPC_StatsComponent.BPC_StatsComponent_C|GetSpeedLeft (Variables|Default|GetBPC_StatsComponent))
                (:%20%20
                  (CallFunction|Move (Variables|Default|GetPath)))))))))))

(event Custom|RotateWidget
  (bind _widget (Variables|Default|GetWidget))
  (Utilities|FlowControl|FlipFlop
    (:A
      (Transformation|SetWorldRotation _widget "90.000000,180.000000,0.000000" false false))
    (:B
      (Transformation|SetWorldRotation _widget "90.000000,0.000000,0.000000" false false))))

(event Custom|OnClicked_Event
  (params (TouchedActor :type Actor%20Object%20Reference) (ButtonPressed :type Key%20Structure :default "None"))
  (Development|PrintString "OnClicked")
  (CallFunction|EventPlayAnim "(X=96.000000,Y=128.000000)")
  (Transformation|SetRelativeLocation (Variables|Default|GetWidget) "0.000000,0.000000,5.000000" false false))

(event Custom|Event%20Play%20Anim
  (params (DesiredSize :type Vector%202D%20Structure))
  (bind _widget (Variables|Default|GetWidget))
  (Variables|Default|SetDesired DesiredSize)
  (Utilities|FlowControl|Gate true) ; enters at Open
)

(event Custom|Event%20Finish%20Anim
  (bind _widget (Variables|Default|GetWidget))
  (Utilities|FlowControl|Gate true) ; enters at Close
)

(event Custom|SetMaskAttack
  (params (Mask :type Array%20of%20Int%20Point%20Structures))
  (bind _output_get (Variables|Default|SetMaskAttack Mask))
  (if (Utilities|Array|IsEmpty _output_get)
    (Variables|Default|SetMaskAttack (Utilities|Array|MakeArray (Utilities|Struct|MakeIntPoint 0 1) (Utilities|Struct|MakeIntPoint 1 0) (Utilities|Struct|MakeIntPoint 0 -1) (Utilities|Struct|MakeIntPoint -1 0)))))

(event Custom|TakeDamage
  (params (Value :type Integer))
  (bind _new_health (Default|TakeDamage (Variables|Default|GetBPC_StatsComponent) Value))
  (bind _aswbp_card (Utilities|Casting|CastToWBP_Card (UserInterface|GetWidget (Variables|Default|GetWidget))))
  (Default|UpdateCardStats _aswbp_card 0 self)
  (if (<= _new_health 0)
    (Variables|/Game/_CardfieldPrototype/TestingPlayground/Filip/Slot/BP_Slot.BP_Slot_C|SetCard (Variables|Default|GetmySlot) 0)
    (Actor|DestroyActor)))

(event Custom|OnHover
  (params (TouchedActor :type Actor%20Object%20Reference))
  (bind _returnvalue (Game|GetPlayerController 0))
  (bind _array (Utilities|Array|MakeArray "ObjectTypeQuery4"))
  (bind (_hitresult _returnvalue_2) (Class|PlayerController|GetHitResultUnderCursorforObjects _returnvalue _array false))
  (Development|PrintString "Hover")
  (Utilities|FlowControl|Delay 0.75)
  (if _returnvalue_2
    (if (== (.HitActor (Collision|BreakHitResult _hitresult)) self)
      (bind _aspc_controller_filip (Utilities|Casting|CastToPC_Controller_Filip (Game|GetPlayerController 0)))
      (switch Utilities|FlowControl|Switch|SwitchonE_ControllerState (Variables|/Game/_CardfieldPrototype/TestingPlayground/Filip/PC_Controller_Filip.PC_Controller_Filip_C|GetState _aspc_controller_filip)
        (:NewEnumerator0
          (CallFunction|EventPlayAnim "(X=192.000000,Y=256.000000)")
          (Transformation|AddRelativeLocation (Variables|Default|GetWidget) "0.000000,0.000000,5.000000" false false)
          (Variables|/Game/_CardfieldPrototype/TestingPlayground/Filip/PC_Controller_Filip.PC_Controller_Filip_C|SetState _aspc_controller_filip "NewEnumerator6"))))))

(event Custom|OnUnhover
  (params (TouchedActor :type Actor%20Object%20Reference))
  (bind _aspc_controller_filip (Utilities|Casting|CastToPC_Controller_Filip (Game|GetPlayerController 0)))
  (switch Utilities|FlowControl|Switch|SwitchonE_ControllerState (Variables|/Game/_CardfieldPrototype/TestingPlayground/Filip/PC_Controller_Filip.PC_Controller_Filip_C|GetState _aspc_controller_filip)
    (:NewEnumerator6
      (CallFunction|EventPlayAnim "(X=96.000000,Y=128.000000)")
      (Transformation|AddRelativeLocation (Variables|Default|GetWidget) "0.000000,0.000000,-5.000000" false false)
      (switch Utilities|FlowControl|Switch|SwitchonE_ControllerState (Variables|/Game/_CardfieldPrototype/TestingPlayground/Filip/PC_Controller_Filip.PC_Controller_Filip_C|GetState _aspc_controller_filip)
        (:NewEnumerator6
          (Variables|/Game/_CardfieldPrototype/TestingPlayground/Filip/PC_Controller_Filip.PC_Controller_Filip_C|SetState _aspc_controller_filip "NewEnumerator0"))))))

(event EventBeginPlay
  (bind _aswbp_card (Utilities|Casting|CastToWBP_Card (UserInterface|GetWidget (Variables|Default|GetWidget))))
  (Default|UpdateCardStats _aswbp_card (Variables|Default|GetStats))
  (bind _aspc_controller_filip (Utilities|Casting|CastToPC_Controller_Filip (Game|GetPlayerController 0)))
  (EventDispatchers|BindEventtoOnPlayerChange _aspc_controller_filip (EventDispatchers|CreateEvent :!event Custom|RotateWidget))
  (CallFunction|SetMaskAttack)
  (Default|InitStats (Variables|Default|GetBPC_StatsComponent) (Variables|Default|GetStats))
  (EventDispatchers|AssignOnBeginCursorOver (EventDispatchers|CreateEvent :!event Custom|OnHover))
  (EventDispatchers|AssignOnEndCursorOver (EventDispatchers|CreateEvent :!event Custom|OnUnhover))
  (EventDispatchers|AssignOnClicked (delegate Custom|OnClicked_Event)))

(event EventTick
  (params (DeltaSeconds :type Float%20%28single-precision%29))
  (bind _widget (Variables|Default|GetWidget))
  (Utilities|FlowControl|Gate true
    (:Exit
      (if (Utilities|Operators|EqualEqual (Class|WidgetComponent|GetDrawSize (Variables|Default|GetWidget)) (Variables|Default|GetDesired) 0.1)
        (CallFunction|EventFinishAnim)
        (else
          (Class|WidgetComponent|SetDrawSize _widget (Class|KismetMathLibrary|Vector2DInterpto (Class|WidgetComponent|GetDrawSize _widget) (Variables|Default|GetDesired) (Utilities|Time|GetWorldDeltaSeconds) 1e+01)))))))

(fn ConstructionScript)