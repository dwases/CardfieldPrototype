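; BP_BravePatient is a passive card ability that raises the owner's Defense and Speed when it takes damage.
; On Initiate it binds GainBoost to the owner card's take-damage event.
; Each positive hit that finds current Health below the base value adds one to both stats in BPCStatsComponent, with no stacking limit.
; LoseBoost reverses one step, but nothing in this Blueprint calls it.
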(event Custom|GainBoost
  (params (DamageValue :type Integer))
  (bind _ownercard (Variables|Default|GetOwnerCard))
  (bind _bpc_statscomponent (Variables|/Game/_CardfieldPrototype/TestingPlayground/Filip/Card/BP_Card.BP_Card_C|GetBPC_StatsComponent _ownercard))
  (bind _stats (Variables|/Game/_CardfieldPrototype/TestingPlayground/Filip/Card/BPC_StatsComponent.BPC_StatsComponent_C|GetStats _bpc_statscomponent))
  (bind (_defense _speed) (Utilities|Struct|BreakS_CardStats _stats))
  (if (> DamageValue 0)
    (if (< (CallFunction|GetOwnerCurrentHP) (CallFunction|GetOwnerMaxHP))
      (Development|PrintString "brave patient buff activated")
      (Utilities|Struct|SetmembersinS_CardStats _stats (+ _defense 1) (+ _speed 1)))))

(event Custom|LoseBoost
  (bind _ownercard (Variables|Default|GetOwnerCard))
  (bind _bpc_statscomponent (Variables|/Game/_CardfieldPrototype/TestingPlayground/Filip/Card/BP_Card.BP_Card_C|GetBPC_StatsComponent _ownercard))
  (bind _stats (Variables|/Game/_CardfieldPrototype/TestingPlayground/Filip/Card/BPC_StatsComponent.BPC_StatsComponent_C|GetStats _bpc_statscomponent))
  (bind (_defense _speed) (Utilities|Struct|BreakS_CardStats _stats))
  (Utilities|Struct|SetmembersinS_CardStats _stats (+ _defense -1) (+ _speed -1)))

(event EventInitiate
  (|CallParentFunction)
  (Development|PrintString "brave patient listening activated")
  (EventDispatchers|BindEventtoOnTakeDamage (Variables|Default|GetOwnerCard) (delegate Custom|GainBoost)))

(fn ConstructionScript
  (|CallParentFunction))

(fn GetOwnerCurrentHP
  (return (Utilities|Struct|BreakS_CardStats (Variables|/Game/_CardfieldPrototype/TestingPlayground/Filip/Card/BPC_StatsComponent.BPC_StatsComponent_C|GetStats (Variables|/Game/_CardfieldPrototype/TestingPlayground/Filip/Card/BP_Card.BP_Card_C|GetBPC_StatsComponent (Variables|Default|GetOwnerCard))))))

(fn GetOwnerMaxHP
  (return (Utilities|Struct|BreakS_CardStats (Variables|/Game/_CardfieldPrototype/TestingPlayground/Filip/Card/CardDataAssets/Units/PDA_UnitStats.PDA_UnitStats_C|GetStats (Variables|/Game/_CardfieldPrototype/TestingPlayground/Filip/Card/BP_Card.BP_Card_C|GetStats (Variables|Default|GetOwnerCard))))))