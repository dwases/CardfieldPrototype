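; BP_HUD_FILIP is a HUD Blueprint in the Cardfield prototype's testing playground that creates and holds UI widgets.
; On BeginPlay it adds the main HUD, resource choice window and backpack widgets to the viewport, storing each in a variable, with the backpack hidden.
; Two events show and hide the resource choice window by toggling its visibility; the file has no logic to reveal the backpack.
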(event Custom|HideResourceChoiceWindow
  (Widget|SetVisibility (Variables|Default|GetResourceChoiceWindow) "Hidden"))

(event Custom|ShowResourceChoiceWindow
  (Widget|SetVisibility (Variables|Default|GetResourceChoiceWindow) "Visible"))

(event EventBeginPlay
  (bind _returnvalue (UserInterface|CreateWidget "/Game/_CardfieldPrototype/TestingPlayground/Filip/HUD/WBP_HUD_Filip.WBP_HUD_Filip_C"))
  (Variables|Default|SetHUD _returnvalue)
  (UserInterface|Viewport|AddtoViewport _returnvalue 0)
  (bind _returnvalue_2 (UserInterface|CreateWidget "/Game/_CardfieldPrototype/TestingPlayground/Filip/HUD/WBP_ResourceChoiceWindow.WBP_ResourceChoiceWindow_C"))
  (bind _output_get (Variables|Default|SetResourceChoiceWindow _returnvalue_2))
  (UserInterface|Viewport|AddtoViewport _output_get 0)
  (bind _returnvalue_3 (UserInterface|CreateWidget "/Game/_CardfieldPrototype/TestingPlayground/Filip/HUD/WBP_Backpack.WBP_Backpack_C"))
  (bind _output_get_2 (Variables|Default|SetBackpackUI _returnvalue_3))
  (Widget|SetVisibility _output_get_2 "Hidden")
  (UserInterface|Viewport|AddtoViewport _output_get_2 0))

(fn ConstructionScript)