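; BP_SquareGrid is a prototype actor that lays out a flat rectangular grid of tiles.
; Its construction script loops over the X and Y grid dimensions and adds one instance to the ISMTiles instanced static mesh component per cell.
; A spacing variable sets each tile's position, and separate XY and Z multipliers set its scale.
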(fn ConstructionScript
  (bind _xytilesizemultiplier (Variables|Tile|GetXYTileSizeMultiplier))
  (for _index (range 0 (- (Variables|Grid|GetXGridDimension) 1))
    (for _index_2 (range 0 (- (Variables|Grid|GetYGridDimension) 1))
      (Components|InstancedStaticMesh|AddInstance (Variables|Default|GetISM_Tiles) (Math|Transform|MakeTransform (Math|Vector|MakeVector (Math|Conversions|ToFloat(Integer) (* _index (Variables|Tile|GetDistanceBetweenTiles))) (Math|Conversions|ToFloat(Integer) (* _index_2 (Variables|Tile|GetDistanceBetweenTiles))) 0.0) "0, 0, 0" (Math|Vector|MakeVector _xytilesizemultiplier _xytilesizemultiplier (Variables|Tile|GetZTileSizeMultiplier))) false))))