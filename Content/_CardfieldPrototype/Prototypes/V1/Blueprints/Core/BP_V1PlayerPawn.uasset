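; Prototype player pawn that manages a card deck, hand and discard pile as integer arrays.
; BeginPlay fills BaseDeck with sequential numbers as cards.
; The Draw event adds a zero to FallenDeck for each held card, clears the hand, then moves random cards from BaseDeck into it if the deck is not empty.
; Debug prints include the hand size every Tick.
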(event Custom|Draw
  (for _array_element (Variables|Default|GetBaseHand)
    (Utilities|Array|Add (Variables|Default|GetFallenDeck) 0))
  (Utilities|Array|Clear (Variables|Default|GetBaseHand))
  (if (not (Utilities|Array|IsEmpty (Variables|Default|GetBaseDeck)))
    (Utilities|FlowControl|ForLoopwithBreak 0 4
      (:LoopBody
        (bind _output_get (Variables|Default|SetTempRandomCard (.OutItem (Utilities|Array|Random (Variables|Default|GetBaseDeck)))))
        (Utilities|Array|Add (Variables|Default|GetBaseHand) _output_get)
        (Utilities|Array|RemoveItem (Variables|Default|GetBaseDeck) _output_get))
      (:Completed
        (Development|PrintString "Hello")))))

(event EventBeginPlay
  (bind _index (Utilities|FlowControl|ForLoopwithBreak 0 49)
    (:LoopBody
      (Utilities|Array|Add (Variables|Default|GetBaseDeck) (+ _index 1)))
    (:Completed
      (Development|PrintString "Hello"))))

(event EventTick
  (params (DeltaSeconds :type Float%20%28single-precision%29))
  (Development|PrintString (Utilities|String|ToString(Integer) (Utilities|Array|Length (Variables|Default|GetBaseHand)))))

(fn ConstructionScript)